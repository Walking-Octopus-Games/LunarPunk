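; Game instance for LunarPunk that manages level progression and menu navigation logic, and applies a shadow quality setting on Init.
; GoToNextLevel and GoToLevel look up names in the Levels array, stop menu logic, then update the current index and open the level if the name is valid.
; StartMenuLogic lazily spawns or reuses a BP_MenuLogic actor, passing it widgets and setting initial button focus, while StopMenuLogic just disables its tick.
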(event Custom|Go%20To%20Level
  (params (Level :type Integer))
  ;[1 1 1] Open Given Level
  (CallFunction|StopMenuLogic)
  (bind _levelname (CallFunction|GetLevelName Level))
  (if (Utilities|Name|NotEqual(Name) _levelname "None")
    (Variables|Default|SetCurrentLevelIndex Level)
    (Game|OpenLevel(byName) _levelname)))

(event Custom|Go%20To%20Next%20Level
  ;[1 1 1] Go to next level
  (CallFunction|StopMenuLogic)
  (bind _levelname (CallFunction|GetLevelName (+ (Variables|Default|GetCurrentLevelIndex) 1)))
  (if (Utilities|Name|NotEqual(Name) _levelname "None")
    (Variables|Default|SetCurrentLevelIndex (+ (Variables|Default|GetCurrentLevelIndex) 1))
    (Game|OpenLevel(byName) _levelname)))

(event EventInit
  (bind _returnvalue (Settings|GetGameUserSettings))
  (Class|GameUserSettings|SetShadowQuality _returnvalue (Variables|Default|GetShadow%20Quality)))

(fn GetLevelName
  (params (Level :type Integer))
  (bind _levels (Variables|Default|GetLevels))
  (if (Utilities|Array|IsValidIndex _levels Level)
    (return (Utilities|Array|Get(acopy) _levels Level))
    (else
      (return "None"))))

(fn StartMenuLogic
  (params (WidgetsArray :type Array%20of%20Widget%20Object%20References))
  (Utilities|IsValid (Variables|Default|GetMenuLogic)
    (:Is%20Valid
      (Actor|Tick|SetActorTickEnabled (Variables|Default|GetMenuLogic) true)
      (Variables|/Game/Blueprints/HUD/BP_MenuLogic.BP_MenuLogic_C|SetWidgetsArray (Variables|Default|GetMenuLogic) WidgetsArray)
      (Default|InitialFocusedButtonSet (Variables|Default|GetMenuLogic)))
    (:Is%20Not%20Valid
      (bind _returnvalue (Game|SpawnActorfromClass "/Game/Blueprints/HUD/BP_MenuLogic.BP_MenuLogic_C" (Math|Transform|MakeTransform "0, 0, 0" "0, 0, 0" "1,1,1") "Undefined" 0 0))
      (Variables|Default|SetMenuLogic _returnvalue)
      (Variables|/Game/Blueprints/HUD/BP_MenuLogic.BP_MenuLogic_C|SetWidgetsArray _returnvalue WidgetsArray)
      (Default|InitialFocusedButtonSet _returnvalue))))

(fn StopMenuLogic
  (bind _menulogic (Variables|Default|GetMenuLogic))
  (Utilities|IsValid _menulogic
    (:Is%20Valid
      (Actor|Tick|SetActorTickEnabled _menulogic))))