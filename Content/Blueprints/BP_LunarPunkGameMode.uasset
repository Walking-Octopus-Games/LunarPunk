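; Game mode for LunarPunk that runs level flow: preparation, gameplay start, pause, game over, restart and return to menu.
; Preparation optionally plays a hold-to-skip cinematic under slowed time dilation with compensated play rate, then opens turret selection or starts gameplay.
; Gameplay start spawns selected turrets, grants upgrades, adds a music layer and applies GameInstance settings.
; Events also drive HUD health and a timeline-faded damage effect.
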(event Custom|PlayerDeath
  (bind _returnvalue (Game|GetPlayerController 0))
  (Audio|PlaySound2D 0 1.0 1.0 0.0 0 0)
  (Utilities|FlowControl|Delay 5.0)
  (Game|SetGamePaused true)
  (Variables|/Script/Engine.PlayerController|SetbShowMouseCursor _returnvalue true)
  (bind _asbp_hud (Utilities|Casting|CastToBP_HUD (HUD|GetHUD _returnvalue)))
  (Default|ShowGameOver _asbp_hud))

(event Custom|Finished%20Cinematic
  ;[1 1 1] Play Cinematic
  (bind _asbp_player_controller (Utilities|Casting|CastToBP_PlayerController (Game|GetPlayerController 0)))
  (Class|LunarPunkPlayerController|SetCutsceneMode _asbp_player_controller false)
  (Default|ToggleSkipCutsceneWidget (stale Custom|PlayCinematic _asbp_hud) false)
  (EventDispatchers|UnbindEventfromSkipCinematic _asbp_player_controller (delegate Custom|Skip%20Cinematic))
  (bind _asbp_camera_manager (Utilities|Casting|CastToBP_CameraManager (Game|GetPlayerCameraManager 0)))
  (Class|CameraManager|SetIsCinematicPlaying _asbp_camera_manager false)
  (Utilities|Time|SetGlobalTimeDilation (Variables|Level|GetDefaultTimeDilation))
  (CallFunction|OnCinematicFinished))

(event Custom|Skip%20Timer%20Finished
  ;[1 1 1] Play Cinematic
  (Class|MovieSceneSequencePlayer|GotoEndandStop (stale Custom|PlayCinematic _returnvalue_2))
  (bind _asbp_player_controller (Utilities|Casting|CastToBP_PlayerController (Game|GetPlayerController 0)))
  (Class|LunarPunkPlayerController|SetCutsceneMode _asbp_player_controller false)
  (Default|ToggleSkipCutsceneWidget (stale Custom|PlayCinematic _asbp_hud) false)
  (EventDispatchers|UnbindEventfromSkipCinematic _asbp_player_controller (delegate Custom|Skip%20Cinematic))
  (bind _asbp_camera_manager (Utilities|Casting|CastToBP_CameraManager (Game|GetPlayerCameraManager 0)))
  (Class|CameraManager|SetIsCinematicPlaying _asbp_camera_manager false)
  (Utilities|Time|SetGlobalTimeDilation (Variables|Level|GetDefaultTimeDilation))
  (CallFunction|OnCinematicFinished))

(event Custom|Start
  (CallFunction|StartLevelGameplay))

(event Custom|Show%20Selection%20Menu
  ;[1 1 1] Open selection menu
  (Game|SetGamePaused true)
  (bind _asbp_hud (Utilities|Casting|CastToBP_HUD (HUD|GetHUD (Game|GetPlayerController 0))))
  (Default|ShowTurretSelectionMenu _asbp_hud))

(event Custom|PauseGame
  (bind _returnvalue (Game|GetPlayerController 0))
  (Game|SetGamePaused true)
  (Variables|/Script/Engine.PlayerController|SetbShowMouseCursor _returnvalue true)
  (bind _asbp_hud (Utilities|Casting|CastToBP_HUD (HUD|GetHUD _returnvalue)))
  (Default|ShowPause _asbp_hud))

(event Custom|ResetActualLevel
  (Game|SetGamePaused false)
  (bind _returnvalue (Game|GetCurrentLevelName true))
  (Game|OpenLevel(byName) (Utilities|String|StringToName _returnvalue)))

(event Custom|Level2Preparation
  (EventDispatchers|BindEventtoEndGameModeInitializeEvent (delegate Custom|Start)))

(event Custom|GoToStartMenu
  (Game|SetGamePaused true)
  (Variables|/Script/Engine.PlayerController|SetbShowMouseCursor (Game|GetPlayerController 0) true)
  (bind _returnvalue (Game|GetCurrentLevelName true))
  (if (Utilities|String|Contains _returnvalue "test")
    (Game|OpenLevel(byName) "StartTestMaps")
    (else
      (Game|OpenLevel(byName) "StartDemoHito2Map"))))

(event Custom|ShowLevelPreparation
  (params (PlayCinematic :type Boolean) (LevelSequence :type Level%20Sequence%20Object%20Reference) (IsSelectionEnabled :type Boolean))
  ;[1 1 1] Prepare Level
  (EventDispatchers|BindEventtoEndGameModeInitializeEvent (delegate Custom|ShowCinematicAndMenu)))

(event Custom|StartLevelGameplay
  (bind _returnvalue (Game|GetPlayerController 0))
  ;[1 1 1] Start Level Gameplay
  (CallFunction|AssignSoundstoManager)
  (CallFunction|SetTurretsHelperIcons true)
  (CallFunction|AddLayerMusic)
  (bind _asbp_hud (Utilities|Casting|CastToBP_HUD (HUD|GetHUD _returnvalue)))
  (Class|HUDManager|TogglePlayerHUDVisibility _asbp_hud true)
  (CallFunction|PreparePlayer)
  (Game|SetGamePaused false)
  (Input|SetInputModeGameandUI _returnvalue 0 "DoNotLock" false)
  (CallFunction|InitializeValuesfromGameInstance)
  (Default|CallGameplayStarted))

(event Custom|Skip%20Cinematic
  (params (IsPressed :type Boolean))
  ;[1 1 1] Play Cinematic
  (if IsPressed
    (bind _returnvalue (Utilities|Time|SetTimerbyEvent (delegate Custom|Skip%20Timer%20Finished) (* (Class|GameplayStatics|GetGlobalTimeDilation) (Variables|Level|GetSkipTime))))
    (else
      (Utilities|Time|PauseTimerbyHandle _returnvalue))))

(event Custom|OnCinematicFinished
  ;[1 1 1] Prepare Level
  (if (stale Custom|ShowLevelPreparation IsSelectionEnabled)
    (CallFunction|ShowSelectionMenu)
    (else
      (CallFunction|StartLevelGameplay))))

(event Custom|ShowCinematicAndMenu
  ;[1 1 1] Prepare Level
  (bind _asbp_hud (Utilities|Casting|CastToBP_HUD (HUD|GetHUD (Game|GetPlayerController 0))))
  (Class|HUDManager|TogglePlayerHUDVisibility _asbp_hud false)
  (Utilities|IsValid (stale Custom|ShowLevelPreparation LevelSequence)
    (:Is%20Valid
      (if (stale Custom|ShowLevelPreparation PlayCinematic)
        (CallFunction|PlayCinematic (stale Custom|ShowLevelPreparation LevelSequence))
        (else
          (if (stale Custom|ShowLevelPreparation IsSelectionEnabled) :!label _label
            (CallFunction|ShowSelectionMenu)
            (else
              (CallFunction|StartLevelGameplay))))))
    (:Is%20Not%20Valid
      (goto _label))))

(event Custom|PlayCinematic
  (params (Level%20Sequence :type Level%20Sequence%20Object%20Reference))
  (bind _returnvalue (Class|GameplayStatics|GetGlobalTimeDilation))
  ;[1 1 1] Play Cinematic
  (CallFunction|SetTurretsHelperIcons false)
  (bind _asbp_camera_manager (Utilities|Casting|CastToBP_CameraManager (Game|GetPlayerCameraManager 0)))
  (Class|CameraManager|SetIsCinematicPlaying _asbp_camera_manager true)
  (Variables|Level|SetDefaultTimeDilation _returnvalue)
  (Utilities|Time|SetGlobalTimeDilation (Variables|Level|GetSlowTimeDilation))
  (bind _returnvalue_2 (Sequencer|Player|CreateLevelSequencePlayer Level%20Sequence (Utilities|Struct|MakeMovieSceneSequencePlaybackSettings false "(Value=0)" (/ 1.0 _returnvalue) 0.0 false false false false true false false false)))
  (bind _asbp_player_controller (Utilities|Casting|CastToBP_PlayerController (Game|GetPlayerController 0)))
  (Class|LunarPunkPlayerController|SetCutsceneMode _asbp_player_controller true)
  (Sequencer|Player|Play _returnvalue_2 :!class /Script/MovieScene.MovieSceneSequencePlayer)
  (EventDispatchers|AssignOnFinished _returnvalue_2 (delegate Custom|Finished%20Cinematic))
  (EventDispatchers|AssignSkipCinematic _asbp_player_controller (delegate Custom|Skip%20Cinematic))
  (bind _asbp_hud (Utilities|Casting|CastToBP_HUD (HUD|GetHUD (Game|GetPlayerController 0))))
  (Default|ToggleSkipCutsceneWidget _asbp_hud true))

(event EventUpdatePlayerLifeinHUD
  (params (Health :type Float%20%28single-precision%29))
  (bind _asbp_hud (Utilities|Casting|CastToBP_HUD (HUD|GetHUD (Game|GetPlayerController 0))))
  (bind _asplayable_character (Utilities|Casting|CastToPlayableCharacter (Game|GetPlayerCharacter 0)))
  (bind _returnvalue (Class|HealthComponent|GetMaxHealth (Variables|/Script/Lunarpunk.PlayableCharacter|GetHealthComponent _asplayable_character)))
  (Default|SetHealthPlayer (Variables|/Game/Blueprints/HUD/BP_HUD.BP_HUD_C|GetHUDPlayerCharacter _asbp_hud) (/ Health _returnvalue)))

(event EventGetTotal
  (params (Enemies :type Integer))
  (Variables|Default|SetMaxEnemies (+ Enemies (Variables|Default|GetMaxEnemies))))

(event EventEndGame
  (bind _returnvalue (Game|GetPlayerController 0))
  (Audio|PlaySound2D 0 1.0 1.0 0.0 0 0)
  (Utilities|FlowControl|Delay 5.0)
  (Game|SetGamePaused true)
  (Variables|/Script/Engine.PlayerController|SetbShowMouseCursor _returnvalue true)
  (bind _asbp_hud (Utilities|Casting|CastToBP_HUD (HUD|GetHUD _returnvalue)))
  (Default|ShowGameOver _asbp_hud))

(event EventRefreshHUDonOpenSector)

(event EventRefreshLifeHUD
  (bind _asbp_hud (Utilities|Casting|CastToBP_HUD (HUD|GetHUD (Game|GetPlayerController 0))))
  (bind _newtrack_0 (Timeline|Timeline_1 Play)
    (:Update
      (Appearance|SetColorandOpacity (Variables|/Game/UI/W_HUD.W_HUD_C|GetDamageEffect (Variables|/Game/Blueprints/HUD/BP_HUD.BP_HUD_C|GetHUDPlayerCharacter _asbp_hud)) (Utilities|Struct|MakeLinearColor 1.0 1.0 1.0 _newtrack_0) :!class /Script/UMG.Image))
    (:Finished
      (if true
        (Timeline|Timeline_1 SetNewTime)))))

(fn ConstructionScript)

(fn SetMenuName
  (params (MenuNameMap :type String))
  (Development|PrintString MenuNameMap true true "(R=0.000000,G=0.660000,B=1.000000,A=1.000000)" 10002.0)
  (bind _output_get (Variables|Default|SetMenuNameMap MenuNameMap))
  (Development|PrintString _output_get true true "(R=1.000000,G=0.201504,B=0.000000,A=1.000000)" 10002.0))

(fn PreparePlayer
  ;[1 1 1] Add upgrades to inventory
  (if (> (Utilities|Array|Length (Variables|Level|GetSelectedUpgrades)) 0)
    (for _array_element (Variables|Level|GetSelectedUpgrades)
      (if (.ReturnValue (Utilities|Map|Find (Variables|/Script/Lunarpunk.UpgradesData|GetUpgrades (Variables|/Script/Lunarpunk.UpgradesManager|GetUpgradesData (Variables|Default|GetUpgradesManager))) _array_element))
        (Class|UpgradesManager|AddUpgrade (Variables|Default|GetUpgradesManager) (.Type (Utilities|Struct|BreakUpgradesDataStruct (.Value (Utilities|Map|Find (Variables|/Script/Lunarpunk.UpgradesData|GetUpgrades (Variables|/Script/Lunarpunk.UpgradesManager|GetUpgradesData (Variables|Default|GetUpgradesManager))) _array_element)))) 1))))
  ;[1 1 1] Add turrets to map
  (if (> (Utilities|Array|Length (Variables|Level|GetSelectedTurrets)) 0)
    (bind _outactors (Actor|GetAllActorsOfClass "/Game/Blueprints/Turrets/AI/BP_TurretWaypoint.BP_TurretWaypoint_C"))
    (bind _array_element_2 (Utilities|Array|ForEachLoopwithBreak _outactors :!label _label)
      (:LoopBody
        (Utilities|IsValid (Variables|/Script/Lunarpunk.TurretWaypoint|GetPrevWaypoint _array_element_2)
          (:Is%20Not%20Valid
            (LocalVariables|SetFirstWaypoint _array_element_2)
            (goto _label Break))))
      (:Completed
        (bind _outactors_2 (Actor|GetAllActorsOfClass "/Game/Blueprints/Turrets/BP_StartingPointTurrets.BP_StartingPointTurrets_C"))
        (Utilities|IsValid (Utilities|Array|Get(acopy) _outactors_2)
          (:Is%20Valid
            (for (_array_element_3 _array_index) (Variables|Level|GetSelectedTurrets)
              (bind _location (Default|GetTurretLocation (Utilities|Array|Get(acopy) _outactors_2) _array_index))
              (switch Utilities|FlowControl|Switch|SwitchonETurretType _array_element_3
                (:MachineGunTurret
                  (bind _returnvalue (Game|SpawnActorfromClass "/Game/Blueprints/Turrets/BP_MachineGunTurret.BP_MachineGunTurret_C" (Math|Conversions|ToTransform(Vector) _location) "AlwaysSpawn" 0 0))
                  (Variables|/Script/Lunarpunk.Turret|SetTargetWaypoint _returnvalue (LocalVariables|GetFirstWaypoint))
                  ;[1 1 1] Meter estas torretas al entity manager e inicializarlas
                  (Class|EntityManager|InitNewTurret (Variables|Default|GetEntityManager) _returnvalue))
                (:AoETurret
                  (bind _returnvalue_2 (Game|SpawnActorfromClass "/Game/Blueprints/Turrets/BP_AreaTurret.BP_AreaTurret_C" (Math|Conversions|ToTransform(Vector) _location) "Undefined" 0 0))
                  (Variables|/Script/Lunarpunk.Turret|SetTargetWaypoint _returnvalue_2 (LocalVariables|GetFirstWaypoint))
                  (Class|EntityManager|InitNewTurret (Variables|Default|GetEntityManager) _returnvalue_2))
                (:HealingTurret
                  (bind _returnvalue_3 (Game|SpawnActorfromClass "/Game/Blueprints/Turrets/BP_HealingTurret.BP_HealingTurret_C" (Math|Conversions|ToTransform(Vector) _location) "Undefined" 0 0))
                  (Variables|/Script/Lunarpunk.Turret|SetTargetWaypoint _returnvalue_3 (LocalVariables|GetFirstWaypoint))
                  (Class|EntityManager|InitNewTurret (Variables|Default|GetEntityManager) _returnvalue_3))))))))))

(fn AddLayerMusic
  (bind _asbp_lunar_punk_game_mode (Utilities|Casting|CastToBP_LunarPunkGameMode (Game|GetGameMode)))
  (Class|AudioManager|AddLayer (Variables|/Script/Lunarpunk.LunarPunkGameMode|GetAudioManager _asbp_lunar_punk_game_mode)))

(fn SetRotationSpeed
  (params (RotationSpeed :type Float%20%28single-precision%29))
  (bind _aslunar_punk_player_controller (Utilities|Casting|CastToLunarPunkPlayerController (Game|GetPlayerController 0)))
  (Variables|/Script/Lunarpunk.LunarPunkPlayerController|SetRotationSpeed _aslunar_punk_player_controller RotationSpeed))

(fn SetTurretsInfo
  (params (bShowTurretsInfo :type Boolean))
  (bind _asbp_lunar_punk_game_mode (Utilities|Casting|CastToBP_LunarPunkGameMode (Game|GetGameMode)))
  (Utilities|IsValid (Variables|/Script/Lunarpunk.LunarPunkGameMode|GetHUDManager _asbp_lunar_punk_game_mode)
    (:Is%20Valid
      (Variables|/Script/Lunarpunk.HUDManager|SetbShowTurretsInfo (Variables|/Script/Lunarpunk.LunarPunkGameMode|GetHUDManager _asbp_lunar_punk_game_mode) bShowTurretsInfo))))

(fn SetAimAssist
  (params (InputPin :type Float%20%28single-precision%29))
  (bind _asplayable_character (Utilities|Casting|CastToPlayableCharacter (Game|GetPlayerCharacter 0))
    (:then
      (Variables|/Script/Lunarpunk.AimAssist|SetAssistAmount (Variables|/Script/Lunarpunk.PlayableCharacter|GetAimAssistComponent _asplayable_character) InputPin))
    (:CastFailed
      _))
  (return InputPin))

(fn SetDamageCheckBox
  (params (InputPin :type Boolean))
  (bind _asbp_lunar_punk_game_mode (Utilities|Casting|CastToBP_LunarPunkGameMode (Game|GetGameMode))
    (:then
      (Utilities|IsValid (Variables|/Script/Lunarpunk.LunarPunkGameMode|GetHUDManager _asbp_lunar_punk_game_mode)
        (:Is%20Valid
          (Class|HUDManager|SetShowDamagePoints (Variables|/Script/Lunarpunk.LunarPunkGameMode|GetHUDManager _asbp_lunar_punk_game_mode) InputPin))
        (:Is%20Not%20Valid
          _)))
    (:CastFailed
      _))
  (return))

(fn InitializeValuesfromGameInstance
  (bind _asbp_lunar_punk_game_instance (Utilities|Casting|CastToBP_LunarPunkGameInstance (Game|GetGameInstance)))
  (CallFunction|SetRotationSpeed (Variables|/Game/Blueprints/BP_LunarPunkGameInstance.BP_LunarPunkGameInstance_C|GetPlayerRotationSpeed _asbp_lunar_punk_game_instance))
  (CallFunction|SetTurretsInfo (Variables|/Game/Blueprints/BP_LunarPunkGameInstance.BP_LunarPunkGameInstance_C|GetShowTurretsInfo _asbp_lunar_punk_game_instance))
  (CallFunction|SetAimAssist (Variables|/Game/Blueprints/BP_LunarPunkGameInstance.BP_LunarPunkGameInstance_C|GetAimAssistValue _asbp_lunar_punk_game_instance))
  (CallFunction|SetDamageCheckBox (Variables|/Game/Blueprints/BP_LunarPunkGameInstance.BP_LunarPunkGameInstance_C|GetShowDamagePoints _asbp_lunar_punk_game_instance)))

(fn SetTurretsHelperIcons
  (params (Show :type Boolean))
  (for _array_element (Variables|/Script/Lunarpunk.EntityManager|GetTurrets (Variables|Default|GetEntityManager))
    (Utilities|IsValid (Variables|/Script/Lunarpunk.Turret|GetPositionHelperIconComponent _array_element)
      (:Is%20Valid
        (if Show
          (Class|PositionHelperIcon|StartPositionIcon (Variables|/Script/Lunarpunk.Turret|GetPositionHelperIconComponent _array_element))
          (else
            (Class|PositionHelperIcon|StopPositionIcon (Variables|/Script/Lunarpunk.Turret|GetPositionHelperIconComponent _array_element)))))
      (:Is%20Not%20Valid
        (if Show
          (Class|PositionHelperIcon|StartPositionIcon (Actor|GetComponentbyClass _array_element "/Game/Blueprints/Turrets/BP_PositionHelperIcon.BP_PositionHelperIcon_C"))
          (else
            (Class|PositionHelperIcon|StopPositionIcon (Actor|GetComponentbyClass _array_element "/Game/Blueprints/Turrets/BP_PositionHelperIcon.BP_PositionHelperIcon_C"))))))))

(fn AssignSoundstoManager
  (Variables|/Script/Lunarpunk.UpgradesManager|SetUpgradeSelectedAudioEvent (Variables|Default|GetUpgradesManager) "/Game/FMOD/Events/Sound_design/Turret_upgrades/Select_turret_upgrade.Select_turret_upgrade"))