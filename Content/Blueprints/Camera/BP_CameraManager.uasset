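; Camera manager that provides an oscillating camera shake and looping gamepad vibration.
; StartShakingCamera sets speeds and angle limits; Tick then lerps Rotation's pitch and yaw, flipping direction at limits around InitialRotation.
; ShakeUP steps pitch by the right/left angle but checks the up/down limit; nothing here sets InitialRotation.
; Vibration runs separately on a looping timer that plays dynamic force feedback at the game instance's VibrationIntensity.
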(event Custom|ShakeRight
  ;[1 1 1] ShakeDirections
  (Variables|Default|SetRotation (Math|Rotator|MakeRotator (.roll (Math|Rotator|Lerp(Rotator) (Variables|Default|GetRotation) (Math|Rotator|MakeRotator (.roll (Variables|Default|GetRotation)) (.pitch (Variables|Default|GetRotation)) (+ (.yaw (Variables|Default|GetRotation)) (Variables|Default|GetUpperRightLeftShakingAngle))) (Variables|Default|GetVelRightLeftRot))) (.pitch (Math|Rotator|Lerp(Rotator) (Variables|Default|GetRotation) (Math|Rotator|MakeRotator (.roll (Variables|Default|GetRotation)) (.pitch (Variables|Default|GetRotation)) (+ (.yaw (Variables|Default|GetRotation)) (Variables|Default|GetUpperRightLeftShakingAngle))) (Variables|Default|GetVelRightLeftRot))) (.yaw (Math|Rotator|Lerp(Rotator) (Variables|Default|GetRotation) (Math|Rotator|MakeRotator (.roll (Variables|Default|GetRotation)) (.pitch (Variables|Default|GetRotation)) (+ (.yaw (Variables|Default|GetRotation)) (Variables|Default|GetUpperRightLeftShakingAngle))) (Variables|Default|GetVelRightLeftRot)))))
  (if (>= (.yaw (Math|Rotator|Lerp(Rotator) (Variables|Default|GetRotation) (Math|Rotator|MakeRotator (.roll (Variables|Default|GetRotation)) (.pitch (Variables|Default|GetRotation)) (+ (.yaw (Variables|Default|GetRotation)) (Variables|Default|GetUpperRightLeftShakingAngle))) (Variables|Default|GetVelRightLeftRot))) (+ (.yaw (Variables|Default|GetInitialRotation)) (Variables|Default|GetUpperRightLeftShakingAngle)))
    (Variables|Default|SetbIsShakingRight false)
    (Variables|Default|SetbIsShakingLeft true)))

(event Custom|ShakeLeft
  ;[1 1 1] ShakeDirections
  (Variables|Default|SetRotation (Math|Rotator|MakeRotator (.roll (Math|Rotator|Lerp(Rotator) (Variables|Default|GetRotation) (Math|Rotator|MakeRotator (.roll (Variables|Default|GetRotation)) (.pitch (Variables|Default|GetRotation)) (+ (.yaw (Variables|Default|GetRotation)) (Variables|Default|GetLowerRightLeftShakingAngle))) (Variables|Default|GetVelRightLeftRot))) (.pitch (Math|Rotator|Lerp(Rotator) (Variables|Default|GetRotation) (Math|Rotator|MakeRotator (.roll (Variables|Default|GetRotation)) (.pitch (Variables|Default|GetRotation)) (+ (.yaw (Variables|Default|GetRotation)) (Variables|Default|GetLowerRightLeftShakingAngle))) (Variables|Default|GetVelRightLeftRot))) (.yaw (Math|Rotator|Lerp(Rotator) (Variables|Default|GetRotation) (Math|Rotator|MakeRotator (.roll (Variables|Default|GetRotation)) (.pitch (Variables|Default|GetRotation)) (+ (.yaw (Variables|Default|GetRotation)) (Variables|Default|GetLowerRightLeftShakingAngle))) (Variables|Default|GetVelRightLeftRot)))))
  (if (<= (.yaw (Math|Rotator|Lerp(Rotator) (Variables|Default|GetRotation) (Math|Rotator|MakeRotator (.roll (Variables|Default|GetRotation)) (.pitch (Variables|Default|GetRotation)) (+ (.yaw (Variables|Default|GetRotation)) (Variables|Default|GetLowerRightLeftShakingAngle))) (Variables|Default|GetVelRightLeftRot))) (+ (.yaw (Variables|Default|GetInitialRotation)) (Variables|Default|GetLowerRightLeftShakingAngle)))
    (Variables|Default|SetbIsShakingRight true)
    (Variables|Default|SetbIsShakingLeft false)))

(event Custom|ShakeUP
  ;[1 1 1] ShakeDirections
  (Variables|Default|SetRotation (Math|Rotator|MakeRotator (.roll (Math|Rotator|Lerp(Rotator) (Variables|Default|GetRotation) (Math|Rotator|MakeRotator (.roll (Variables|Default|GetRotation)) (+ (.pitch (Variables|Default|GetRotation)) (Variables|Default|GetUpperRightLeftShakingAngle)) (.yaw (Variables|Default|GetRotation))) (Variables|Default|GetVelUpDownRot))) (.pitch (Math|Rotator|Lerp(Rotator) (Variables|Default|GetRotation) (Math|Rotator|MakeRotator (.roll (Variables|Default|GetRotation)) (+ (.pitch (Variables|Default|GetRotation)) (Variables|Default|GetUpperRightLeftShakingAngle)) (.yaw (Variables|Default|GetRotation))) (Variables|Default|GetVelUpDownRot))) (.yaw (Math|Rotator|Lerp(Rotator) (Variables|Default|GetRotation) (Math|Rotator|MakeRotator (.roll (Variables|Default|GetRotation)) (+ (.pitch (Variables|Default|GetRotation)) (Variables|Default|GetUpperRightLeftShakingAngle)) (.yaw (Variables|Default|GetRotation))) (Variables|Default|GetVelUpDownRot)))))
  (if (>= (.pitch (Math|Rotator|Lerp(Rotator) (Variables|Default|GetRotation) (Math|Rotator|MakeRotator (.roll (Variables|Default|GetRotation)) (+ (.pitch (Variables|Default|GetRotation)) (Variables|Default|GetUpperRightLeftShakingAngle)) (.yaw (Variables|Default|GetRotation))) (Variables|Default|GetVelUpDownRot))) (+ (.pitch (Variables|Default|GetInitialRotation)) (Variables|Default|GetUpperUpDownShakingAngle)))
    (Variables|Default|SetbIsShakingUp false)
    (Variables|Default|SetbIsShakingDown true)))

(event Custom|ShakeDown
  ;[1 1 1] ShakeDirections
  (Variables|Default|SetRotation (Math|Rotator|MakeRotator (.roll (Math|Rotator|Lerp(Rotator) (Variables|Default|GetRotation) (Math|Rotator|MakeRotator (.roll (Variables|Default|GetRotation)) (+ (.pitch (Variables|Default|GetRotation)) (Variables|Default|GetLowerUpDownShakingAngle)) (.yaw (Variables|Default|GetRotation))) (Variables|Default|GetVelUpDownRot))) (.pitch (Math|Rotator|Lerp(Rotator) (Variables|Default|GetRotation) (Math|Rotator|MakeRotator (.roll (Variables|Default|GetRotation)) (+ (.pitch (Variables|Default|GetRotation)) (Variables|Default|GetLowerUpDownShakingAngle)) (.yaw (Variables|Default|GetRotation))) (Variables|Default|GetVelUpDownRot))) (.yaw (Math|Rotator|Lerp(Rotator) (Variables|Default|GetRotation) (Math|Rotator|MakeRotator (.roll (Variables|Default|GetRotation)) (+ (.pitch (Variables|Default|GetRotation)) (Variables|Default|GetLowerUpDownShakingAngle)) (.yaw (Variables|Default|GetRotation))) (Variables|Default|GetVelUpDownRot)))))
  (if (<= (.pitch (Math|Rotator|Lerp(Rotator) (Variables|Default|GetRotation) (Math|Rotator|MakeRotator (.roll (Variables|Default|GetRotation)) (+ (.pitch (Variables|Default|GetRotation)) (Variables|Default|GetLowerUpDownShakingAngle)) (.yaw (Variables|Default|GetRotation))) (Variables|Default|GetVelUpDownRot))) (+ (.pitch (Variables|Default|GetInitialRotation)) (Variables|Default|GetLowerUpDownShakingAngle)))
    (Variables|Default|SetbIsShakingUp true)
    (Variables|Default|SetbIsShakingDown false)))

(event Custom|StartGamepadVibration
  ;[1 1 1] Gamepad vibration
  (Utilities|Time|ClearandInvalidateTimerbyHandle (Variables|Default|GetGamePadVibrationTimer))
  (bind _returnvalue (Utilities|Time|SetTimerbyEvent (delegate Custom|Vibrate) 0.5 true))
  (Variables|Default|SetGamePadVibrationTimer _returnvalue))

(event Custom|Vibrate
  ;[1 1 1] Gamepad vibration
  (bind _asbp_lunar_punk_game_instance (Utilities|Casting|CastToBP_LunarPunkGameInstance (Game|GetGameInstance)))
  (Game|Feedback|PlayDynamicForceFeedback (Game|GetPlayerController 0) (Variables|/Game/Blueprints/BP_LunarPunkGameInstance.BP_LunarPunkGameInstance_C|GetVibrationIntensity _asbp_lunar_punk_game_instance) 0.4 true true true true))

(event Custom|StopGamepadVibration
  ;[1 1 1] Gamepad vibration
  (Utilities|Time|ClearandInvalidateTimerbyHandle (Variables|Default|GetGamePadVibrationTimer)))

(event EventBeginPlay)

(event Collision|EventActorBeginOverlap
  (params (OtherActor :type Actor%20Object%20Reference)))

(event EventTick
  (params (DeltaSeconds :type Float%20%28single-precision%29))
  (if (and (Variables|Default|GetbShakeEffectEnabled) (Variables|Default|GetbIsShaking))
    (Utilities|FlowControl|Sequence
      (:then_0
        (if (Variables|Default|GetbIsShakingRight)
          (CallFunction|ShakeRight)))
      (:then_1
        (if (Variables|Default|GetbIsShakingLeft)
          (CallFunction|ShakeLeft)))
      (:then_2
        (if (Variables|Default|GetbIsShakingUp)
          (CallFunction|ShakeUP)))
      (:then_3
        (if (Variables|Default|GetbIsShakingDown)
          (CallFunction|ShakeDown))))))

(event EventStartShakingCamera
  (params (UpDownRotationSpeed :type Float%20%28single-precision%29) (RightLeftRotationSpeed :type Float%20%28single-precision%29) (UpDownAngle :type Float%20%28single-precision%29) (RightLeftAngle :type Float%20%28single-precision%29) (ShouldVibrate :type Boolean))
  ;[1 1 1] Start/Stop Shake
  (CallFunction|SetShakeParams UpDownRotationSpeed RightLeftRotationSpeed UpDownAngle RightLeftAngle)
  (CallFunction|SetShakingEnabled true))

(event EventStopShakingCamera
  ;[1 1 1] Start/Stop Shake
  (CallFunction|SetShakingEnabled false))

(fn ConstructionScript)

(fn SetShakeParams
  (params (UpDownRotationSpeed :type Float%20%28single-precision%29) (RightLeftRotationSpeed :type Float%20%28single-precision%29) (UpDownAngle :type Float%20%28single-precision%29) (RghtLeftAngle :type Float%20%28single-precision%29))
  (Variables|Default|SetVelUpDownRot UpDownRotationSpeed)
  (Variables|Default|SetVelRightLeftRot RightLeftRotationSpeed)
  (Variables|Default|SetUpperUpDownShakingAngle UpDownAngle)
  (Variables|Default|SetLowerUpDownShakingAngle (* UpDownAngle -1.0))
  (Variables|Default|SetUpperRightLeftShakingAngle RghtLeftAngle)
  (Variables|Default|SetLowerRightLeftShakingAngle (* RghtLeftAngle -1.0)))

(fn SetShakingEnabled
  (params (Enabled :type Boolean))
  (if Enabled
    (Variables|Default|SetbIsShaking true)
    (Variables|Default|SetbIsShakingRight true)
    (Variables|Default|SetbIsShakingLeft false)
    (Variables|Default|SetbIsShakingUp true)
    (Variables|Default|SetbIsShakingDown false)
    (else
      (Variables|Default|SetbIsShaking false)
      (Variables|Default|SetbIsShakingRight false)
      (Variables|Default|SetbIsShakingLeft false)
      (Variables|Default|SetbIsShakingUp false)
      (Variables|Default|SetbIsShakingDown false))))