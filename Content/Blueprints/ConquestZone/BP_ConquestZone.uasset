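; Conquest zone actor that handles the zone's visual feedback, HUD prompts and upward platform movement.
; Player-can-shoot dispatchers toggle the skeletal mesh and the destroy-portal controls, while activation events swap materials on both meshes.
; Rest-phase events animate and refresh the next-wave countdown, adding a choose-fork prompt on forks.
; UpPlatform makes Tick raise the actor by a given distance; dynamic-material opacity code is left unconnected.
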(event Custom|ShowPlayerCanShoot_Event_0
  (bind _asbp_hud (Utilities|Casting|CastToBP_HUD (HUD|GetHUD (Game|GetPlayerController 0))))
  (Default|ShowControlsDestroyPortal (Variables|/Game/Blueprints/HUD/BP_HUD.BP_HUD_C|GetHUDPlayerCharacter _asbp_hud))
  (Rendering|SetVisibility (Variables|Default|GetSkeletalMesh) false false))

(event Custom|HidePlayerCanShoot_Event_0
  (bind _asbp_hud (Utilities|Casting|CastToBP_HUD (HUD|GetHUD (Game|GetPlayerController 0))))
  (Default|HideControlsDestroyPortal (Variables|/Game/Blueprints/HUD/BP_HUD.BP_HUD_C|GetHUDPlayerCharacter _asbp_hud))
  (Rendering|SetVisibility (Variables|Default|GetSkeletalMesh) true false))

(event Custom|UpPlatform
  (params (Distance :type Float%20%28single-precision%29))
  (Variables|Default|SetDistanceToUp Distance)
  (Variables|Default|SetCurrentDistance 0.0)
  (Variables|Default|SetIsMoving true))

(event EventBeginPlay
  (EventDispatchers|AssignShowPlayerCanShoot (delegate Custom|ShowPlayerCanShoot_Event_0))
  (EventDispatchers|AssignHidePlayerCanShoot (delegate Custom|HidePlayerCanShoot_Event_0)))

(event EventTick
  (params (DeltaSeconds :type Float%20%28single-precision%29))
  (bind _speed (Variables|Default|GetSpeed))
  (bind _returnvalue (* DeltaSeconds _speed))
  (if (Variables|Default|GetIsMoving)
    (Variables|Default|SetCurrentDistance (+ (Variables|Default|GetCurrentDistance) _returnvalue))
    (Transformation|AddActorWorldOffset (Math|Vector|MakeVector 0.0 0.0 _returnvalue))
    (if (>= (Variables|Default|GetCurrentDistance) (Variables|Default|GetDistanceToUp))
      (Variables|Default|SetIsMoving false))))

(event EventShowZoneActivatedEffect
  (Rendering|Material|SetMaterial (Variables|Default|GetConquestMesh) 0 "/Game/Materials/MI_BlueAndroidLamp.MI_BlueAndroidLamp")
  (CallFunction|SetMaterialsEnabled true))

(event EventRemoveZoneActivatedEffect
  (Rendering|Material|SetMaterial (Variables|Default|GetConquestMesh) 0 "/Engine/BasicShapes/BasicShapeMaterial.BasicShapeMaterial")
  (CallFunction|SetMaterialsEnabled false))

(event EventHideTimetoNextWaveinHUD
  (if (Variables|Default|GetbShowingRestingTime)
    (Variables|Default|SetbShowingRestingTime false)
    (bind _asbp_hud (Utilities|Casting|CastToBP_HUD (HUD|GetHUD (Game|GetPlayerController 0))))
    (Utilities|IsValid (Variables|/Game/Blueprints/HUD/BP_HUD.BP_HUD_C|GetHUDPlayerCharacter _asbp_hud)
      (:Is%20Valid
        (UserInterface|Animation|PlayAnimation (Variables|/Game/Blueprints/HUD/BP_HUD.BP_HUD_C|GetHUDPlayerCharacter _asbp_hud) (Variables|/Game/UI/W_HUD.W_HUD_C|GetHideTimeToNextWave (Variables|/Game/Blueprints/HUD/BP_HUD.BP_HUD_C|GetHUDPlayerCharacter _asbp_hud)) 0.0 1 "Forward" 1.0 false)
        (if (Variables|Default|GetIsFork)
          (Widget|SetRenderOpacity (Variables|/Game/UI/W_HUD.W_HUD_C|GetChooseFork (Variables|/Game/Blueprints/HUD/BP_HUD.BP_HUD_C|GetHUDPlayerCharacter _asbp_hud)) 0.0))))))

(event EventRefreshHUDTimetoNextWave
  (bind _asbp_hud (Utilities|Casting|CastToBP_HUD (HUD|GetHUD (Game|GetPlayerController 0))))
  (Utilities|IsValid (Variables|/Game/Blueprints/HUD/BP_HUD.BP_HUD_C|GetHUDPlayerCharacter _asbp_hud)
    (:Is%20Valid
      (Rendering|Components|TextRender|SetText (Variables|/Game/UI/W_HUD.W_HUD_C|GetTimeNextWave (Variables|/Game/Blueprints/HUD/BP_HUD.BP_HUD_C|GetHUDPlayerCharacter _asbp_hud)) (Utilities|Text|ToText(Integer) (Variables|Default|GetCurrentTimeToEndResting))))))

(event EventShowTimetoNextWaveinHUD
  (Variables|Default|SetbShowingRestingTime true)
  (bind _asbp_hud (Utilities|Casting|CastToBP_HUD (HUD|GetHUD (Game|GetPlayerController 0))))
  (Utilities|IsValid (Variables|/Game/Blueprints/HUD/BP_HUD.BP_HUD_C|GetHUDPlayerCharacter _asbp_hud)
    (:Is%20Valid
      (UserInterface|Animation|PlayAnimation (Variables|/Game/Blueprints/HUD/BP_HUD.BP_HUD_C|GetHUDPlayerCharacter _asbp_hud) (Variables|/Game/UI/W_HUD.W_HUD_C|GetShowTimeToNextWave (Variables|/Game/Blueprints/HUD/BP_HUD.BP_HUD_C|GetHUDPlayerCharacter _asbp_hud)) 0.0 1 "Forward" 1.0 false)
      (bind _newtrack_0 (Timeline|Timeline_0 Play)
        (:Update
          (Widget|Transform|SetRenderScale (Variables|/Game/UI/W_HUD.W_HUD_C|GetTextTimeNextWave (Variables|/Game/Blueprints/HUD/BP_HUD.BP_HUD_C|GetHUDPlayerCharacter _asbp_hud)) (Math|Vector2D|MakeVector2D _newtrack_0 _newtrack_0))
          (Widget|Transform|SetRenderScale (Variables|/Game/UI/W_HUD.W_HUD_C|GetTimeNextWave (Variables|/Game/Blueprints/HUD/BP_HUD.BP_HUD_C|GetHUDPlayerCharacter _asbp_hud)) (Math|Vector2D|MakeVector2D _newtrack_0 _newtrack_0))
          (Widget|SetRenderOpacity (Variables|/Game/UI/W_HUD.W_HUD_C|GetTextTimeNextWave (Variables|/Game/Blueprints/HUD/BP_HUD.BP_HUD_C|GetHUDPlayerCharacter _asbp_hud)) 1.0)
          (if (Variables|Default|GetIsFork)
            (Widget|SetRenderOpacity (Variables|/Game/UI/W_HUD.W_HUD_C|GetChooseFork (Variables|/Game/Blueprints/HUD/BP_HUD.BP_HUD_C|GetHUDPlayerCharacter _asbp_hud)) 1.0)))))))

(fn ConstructionScript)

(fn SetMaterialsEnabled
  (params (Enabled :type Boolean))
  (if Enabled
    (Rendering|Material|SetMaterial (Variables|Default|GetSkeletalMesh) 0 "/Game/Materials/PlaceholderTurrets/M_PlaceholderPlayer.M_PlaceholderPlayer")
    (Rendering|Material|SetMaterial (Variables|Default|GetSkeletalMesh) 1 "/Game/Materials/PlaceholderTurrets/M_PlaceholderPlayer.M_PlaceholderPlayer")
    (Rendering|Material|SetMaterial (Variables|Default|GetSkeletalMesh) 2 "/Game/Materials/PlaceholderTurrets/M_PlaceholderPlayer.M_PlaceholderPlayer")
    (Rendering|Material|SetMaterial (Variables|Default|GetSkeletalMesh) 3 "/Game/Materials/PlaceholderTurrets/M_PlaceholderPlayer.M_PlaceholderPlayer")
    (else
      (Rendering|Material|SetMaterial (Variables|Default|GetSkeletalMesh) 0 "/Game/Materials/PlaceholderTurrets/MI_PlaceholderPlayer.MI_PlaceholderPlayer")
      (Rendering|Material|SetMaterial (Variables|Default|GetSkeletalMesh) 1 "/Game/Materials/PlaceholderTurrets/MI_PlaceholderPlayer.MI_PlaceholderPlayer")
      (Rendering|Material|SetMaterial (Variables|Default|GetSkeletalMesh) 2 "/Game/Materials/PlaceholderTurrets/MI_PlaceholderPlayer.MI_PlaceholderPlayer")
      (Rendering|Material|SetMaterial (Variables|Default|GetSkeletalMesh) 3 "/Game/Materials/PlaceholderTurrets/MI_PlaceholderPlayer.MI_PlaceholderPlayer"))))