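; Turret placement platform for conquest zones that previews the available turret types as cycling holograms.
; A looping timer steps through machine gun, healing and area ghost meshes, with timelines fading the opacity of one shared dynamic material.
; Events toggle the ghosts, platform effect and base material for zone activation.
; UpPlatform raises the whole actor by a given distance at constant speed on Tick.
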(event Custom|Event%20Change%20Turret%20Ghost
  (if (Variables|Default|GetUpdateGhost)
    (bind _opacity (Timeline|TurretGhostHide PlayFromStart)
      (:Update
        (Rendering|Material|SetScalarParameterValue (Variables|Default|GetGhostMaterial) "Opacity" _opacity :!class /Script/Engine.MaterialInstanceDynamic))
      (:Finished
        (Rendering|SetVisibility (Utilities|Array|Get(acopy) (Variables|Default|GetGhostMeshes) (Variables|Default|GetGhostIndex)) false true)
        (bind _result (Math|Integer|IncrementInt (Variables|Default|GetGhostIndex))
          (:%20%20
            (if (>= _result (Utilities|Array|Length (Variables|Default|GetGhostMeshes)))
              (Variables|Default|SetGhostIndex 0)
              (bind _opacity_2 (Timeline|TurretGhostShow PlayFromStart)
                (:Update
                  (Rendering|Material|SetScalarParameterValue (Variables|Default|GetGhostMaterial) "Opacity" _opacity_2 :!class /Script/Engine.MaterialInstanceDynamic))
                (:Finished
                  ;[1 1 1] Check a second time in case value changed
                  (if (Variables|Default|GetUpdateGhost)
                    (Rendering|SetVisibility (Utilities|Array|Get(acopy) (Variables|Default|GetGhostMeshes) (Variables|Default|GetGhostIndex)) true true)
                    (Components|Activation|Activate (Variables|Default|GetPlatformEffect) false)
                    (Rendering|SetVisibility (Variables|Default|GetPlatformEffect) true false))))
              (else
                (Timeline|TurretGhostShow PlayFromStart)))))))
    (else
      (bind _result_2 (Math|Integer|IncrementInt (Variables|Default|GetGhostIndex))
        (:%20%20
          (if (>= _result_2 (Utilities|Array|Length (Variables|Default|GetGhostMeshes)))
            (Variables|Default|SetGhostIndex 0)))))))

(event Custom|UpPlatform
  (params (Distance :type Float%20%28single-precision%29))
  (Variables|UpEffect|SetDistanceToUp Distance)
  (Variables|UpEffect|SetCurrentDistance 0.0)
  (Variables|UpEffect|SetIsMoving true))

(event EventTick
  (params (DeltaSeconds :type Float%20%28single-precision%29))
  (bind _speed (Variables|UpEffect|GetSpeed))
  (bind _returnvalue (* DeltaSeconds _speed))
  (if (Variables|UpEffect|GetIsMoving)
    (Variables|UpEffect|SetCurrentDistance (+ (Variables|UpEffect|GetCurrentDistance) _returnvalue))
    (Transformation|AddActorWorldOffset (Math|Vector|MakeVector 0.0 0.0 _returnvalue))
    (if (>= (Variables|UpEffect|GetCurrentDistance) (Variables|UpEffect|GetDistanceToUp))
      (Variables|UpEffect|SetIsMoving false))))

(event EventRemoveZoneActivatedEffect
  (Rendering|Material|SetMaterial (Variables|Default|GetPlaceBase) 0 "/AnimationSharing/AnimSharingRed.AnimSharingRed"))

(event EventShowZoneActivatedEffect
  (Rendering|Material|SetMaterial (Variables|Default|GetPlaceBase) 0 "/Game/Materials/MI_RedAndroidLamp.MI_RedAndroidLamp")
  (Components|Activation|Deactivate (Variables|Default|GetPlatformEffect))
  (Rendering|SetVisibility (Variables|Default|GetPlatformEffect) false false))

(event EventRemoveTurretGhost
  (Variables|Default|SetUpdateGhost false)
  (for _array_element (Variables|Default|GetGhostMeshes)
    (Rendering|SetVisibility _array_element false true)))

(event EventShowTurretGhost
  (Variables|Default|SetUpdateGhost true)
  (Components|Activation|Activate (Variables|Default|GetPlatformEffect) false)
  (Rendering|SetVisibility (Variables|Default|GetPlatformEffect) true false))

(event EventBeginPlay
  (Utilities|Time|SetTimerbyEvent (delegate Custom|Event%20Change%20Turret%20Ghost) (Variables|Default|GetTimeGhostRefresh) true))

(fn ConstructionScript
  (bind _returnvalue (Rendering|Material|CreateDynamicMaterialInstance "/Game/Materials/PlaceholderTurrets/MI_PlaceholderTurrets.MI_PlaceholderTurrets" "None" "None" :!class /Script/Engine.KismetMaterialLibrary))
  (bind _output_get (Variables|Default|SetGhostMaterial _returnvalue))
  (Rendering|Material|SetMaterial (Variables|Default|GetMachineGunBase) 0 _output_get)
  (Rendering|Material|SetMaterial (Variables|Default|GetMachineGunWeapon) 0 _output_get)
  (Rendering|Material|SetMaterial (Variables|Default|GetHealing) 0 _output_get)
  (Rendering|Material|SetMaterial (Variables|Default|GetAreaBase) 0 _output_get)
  (Rendering|Material|SetMaterial (Variables|Default|GetAreaWeapon) 0 _output_get)
  (Variables|Default|SetGhostMeshes (Utilities|Array|MakeArray (Variables|Default|GetMachineGunBase) (Variables|Default|GetHealing) (Variables|Default|GetAreaBase))))