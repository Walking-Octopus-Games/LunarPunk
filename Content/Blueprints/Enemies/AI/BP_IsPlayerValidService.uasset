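; Behavior tree service for enemy AI that, despite its player-validity name, has the EnemyAIController update its next target point on each tick.
; A helper reads the "Player" blackboard object and has the controller check that the actor is valid.
; Another helper requests a random point in a Turret's area.
; The tick event calls neither helper.
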(event EventReceiveTickAI
  (params (OwnerController :type AI%20Controller%20Object%20Reference) (ControlledPawn :type Pawn%20Object%20Reference) (DeltaSeconds :type Float%20%28single-precision%29))
  (bind _asenemy_aicontroller (Utilities|Casting|CastToEnemyAIController OwnerController))
  (Class|EnemyAIController|UpdateNextTargetPoint _asenemy_aicontroller))

(fn UpdateAreaTargetPoint
  (params (self2 :type Enemy%20AI%20Controller%20Object%20Reference) (TurretTarget :type Actor%20Object%20Reference) (Object :type Object%20Object%20Reference))
  (Utilities|Casting|CastToTurret Object)
  (Class|EnemyAIController|GetRandomPointinTurretArea self2 TurretTarget))

(fn CheckifthePlayerIsValid
  (params (Controller :type Object%20Object%20Reference))
  (bind _asenemy_aicontroller (Utilities|Casting|CastToEnemyAIController Controller)
    (:then
      (bind _asactor (Utilities|Casting|CastToActor (AI|Components|Blackboard|GetValueasObject (AI|GetBlackboard _asenemy_aicontroller) (Utilities|String|StringToName "Player"))))
      (bind _returnvalue (Class|EnemyAIController|CheckIstheActorValid _asenemy_aicontroller _asactor)))
    (:CastFailed
      _))
  (return _asenemy_aicontroller _returnvalue _asactor))