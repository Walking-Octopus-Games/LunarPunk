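; Behavior tree service for enemy AI that refreshes the controller's target point.
; Each AI tick casts the owner to EnemyAIController and calls UpdateNextTargetPoint, leaving the logic to the controller.
; Two helper functions, not called by the tick, validate the blackboard TurretTarget actor through the controller and request a random point in a turret's area.
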(event EventReceiveTickAI
  (params (OwnerController :type AI%20Controller%20Object%20Reference) (ControlledPawn :type Pawn%20Object%20Reference) (DeltaSeconds :type Float%20%28single-precision%29))
  (bind _asenemy_aicontroller (Utilities|Casting|CastToEnemyAIController OwnerController))
  (Class|EnemyAIController|UpdateNextTargetPoint _asenemy_aicontroller))

(fn UpdateAreaTargetPoint
  (params (self2 :type Enemy%20AI%20Controller%20Object%20Reference) (TurretTarget :type Actor%20Object%20Reference) (Object :type Object%20Object%20Reference))
  (Utilities|Casting|CastToTurret Object)
  (Class|EnemyAIController|GetRandomPointinTurretArea self2 TurretTarget))

(fn CheckiftheTargetIsValid
  (params (Target :type Actor%20Object%20Reference) (Object :type Object%20Object%20Reference))
  (bind _returnvalue (AI|GetBlackboard Target))
  (bind _returnvalue_2 (Utilities|String|StringToName "TurretTarget"))
  (bind _returnvalue_3 (AI|Components|Blackboard|GetValueasObject _returnvalue _returnvalue_2))
  (bind _asenemy_aicontroller (Utilities|Casting|CastToEnemyAIController Object))
  (bind _asactor (Utilities|Casting|CastToActor _returnvalue_3))
  (bind _returnvalue_4 (Class|EnemyAIController|CheckIstheActorValid _asenemy_aicontroller _asactor))
  (return _returnvalue_3 _asenemy_aicontroller _returnvalue_4 _asactor))