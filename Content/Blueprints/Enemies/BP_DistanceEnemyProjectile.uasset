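; Projectile Blueprint for a distance enemy, defining the visual and audio feedback of its impact.
; SpawnImpactEffect spawns an enlarged hit effect slightly below the given location and tints it from the R, G, B and A variables, sent as a color and as separate RGB float parameters.
; It then plays the enemy impact audio event attached to the root component.
; No movement or collision logic is implemented in these graphs.
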(event EventBeginPlay
  (|CallParentFunction) ; This node is disabled and will not be called.\nDrag off pins to build functionality.
)

(event Collision|EventActorBeginOverlap
  (params (OtherActor :type Actor%20Object%20Reference))
  (|CallParentFunction OtherActor) ; This node is disabled and will not be called.\nDrag off pins to build functionality.
)

(event EventTick
  (params (DeltaSeconds :type Float%20%28single-precision%29))
  (|CallParentFunction DeltaSeconds) ; This node is disabled and will not be called.\nDrag off pins to build functionality.
)

(event EventSpawnImpactEffect
  (params (Location :type Vector :default "0, 0, 0"))
  (bind _r (Variables|Default|GetR))
  (bind _g (Variables|Default|GetG))
  (bind _b (Variables|Default|GetB))
  (bind _returnvalue (Niagara|SpawnSystematLocation "/Game/Particles/FX_HitEffect/FXS_HitEffect.FXS_HitEffect" (- Location "0, 0,20.000000") "0, 0, 0" "2.000000,2.000000,2.000000"))
  (Effects|Components|ParticleSystem|SetColorParameter _returnvalue "Color" (Math|Color|MakeColor _r _g _b (Variables|Default|GetA)))
  (Effects|Components|ParticleSystem|SetFloatParameter _returnvalue "R" _r)
  (Effects|Components|ParticleSystem|SetFloatParameter _returnvalue "G" _g)
  (Effects|Components|ParticleSystem|SetFloatParameter _returnvalue "B" _b)
  (Class|FMODBlueprintStatics|PlayEventAttached "/Game/FMOD/Events/Sound_design/Enemy_attack/impact_Enemy_3.impact_Enemy_3" (Variables|Transformation|GetRootComponent) "None" "0, 0, 0" "KeepRelativeOffset"))

(fn ConstructionScript
  (|CallParentFunction))