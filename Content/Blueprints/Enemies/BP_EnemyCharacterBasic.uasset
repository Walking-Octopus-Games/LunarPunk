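; Basic pooled Razarac enemy character with a health bar, floating damage numbers and colored Niagara impact effects.
; HealthComponent events refresh the health widget, while damage display plays widget animations and a timeline-driven flash across the mesh's dynamic materials.
; On death it drops rewards, deactivates, plays the death animation for a fixed delay, returns to the pool and, unless NonReturnable, notifies the game mode.
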(event ActorDeath(HealthComponent)
  (bind _mesh (Variables|Character|GetMesh))
  (bind _returnvalue (Components|SkeletalMesh|GetAnimInstance _mesh))
  ;[1 1 1] Actor Death
  (Class|DropRewardsComponent|DropRewards (Variables|Default|GetDropRewards))
  (Class|BasicEnemy|DeactivateforDeathAnim)
  (Utilities|IsValid _returnvalue
    (:Is%20Valid
      (bind _asraz_anim (Utilities|Casting|CastToRazAnim _returnvalue))
      (Variables|/Game/Mannequin/Animations/Raz/RazAnim.RazAnim_C|SetIsDead _asraz_anim true)
      (Utilities|FlowControl|Delay 2.0)
      (Variables|/Game/Mannequin/Animations/Raz/RazAnim.RazAnim_C|SetIsDead _asraz_anim false)
      (Class|BasicEnemy|ReturntoPool)
      (if (not (Variables|Default|GetbNonReturnable))
        (bind _asw_enemy_health_with_numbers (Utilities|Casting|CastToW_EnemyHealthWithNumbers (UserInterface|GetUserWidgetObject (Variables|Default|GetHealthWidget))))
        (bind _output_get (Variables|Default|SetHealthWidgetRef _asw_enemy_health_with_numbers))
        (Default|UpdateLifeText _output_get)
        (bind _asbp_enemy_interface (Utilities|Casting|CastToBP_EnemyInterface (Game|GetGameMode)))
        (Default|DestroyEnemy _asbp_enemy_interface)))))

(event UpdateHealth(HealthComponent)
  (params (Health :type Float%20%28single-precision%29))
  (CallFunction|UpdateLifeBar))

(event EventBeginPlay
  (CallFunction|SetMaterials)
  (bind _asw_enemy_health_with_numbers (Utilities|Casting|CastToW_EnemyHealthWithNumbers (UserInterface|GetUserWidgetObject (Variables|Default|GetHealthWidget))))
  (Variables|Default|SetHealthWidgetRef _asw_enemy_health_with_numbers)
  (CallFunction|UpdateLifeBar)
  (bind _asw_enemies_damage (Utilities|Casting|CastToW_EnemiesDamage (UserInterface|GetUserWidgetObject (Variables|Default|GetDamagePointsWidget))))
  (Variables|Default|SetDamagePointsWidgetRef _asw_enemies_damage))

(event Collision|EventActorBeginOverlap
  (params (OtherActor :type Actor%20Object%20Reference)))

(event EventDrawDamageWidget
  (params (DamageReceived :type Float%20%28single-precision%29))
  (bind _returnvalue (Math|Float|Truncate DamageReceived))
  (bind _damagepointswidgetref (Variables|Default|GetDamagePointsWidgetRef))
  (bind _healthwidgetref (Variables|Default|GetHealthWidgetRef))
  ;[1 1 1] Draw Damage points when hittet
  (bind (_text _anim) (Default|GetNextTextandAnim _damagepointswidgetref))
  (Rendering|Components|TextRender|SetText _text (Utilities|Text|ToText(Integer) _returnvalue))
  (UserInterface|Animation|PlayAnimation _damagepointswidgetref _anim 0.0 1 "Forward" 1.0 false)
  (UserInterface|Animation|PlayAnimation _healthwidgetref (Variables|/Game/UI/HealthLifeBars/W_EnemyHealthWithNumbers.W_EnemyHealthWithNumbers_C|GetDamageEffectAnim _healthwidgetref) 0.0 1 "Forward" 1.0 false)
  (if (> _returnvalue 0)
    (bind _newtrack_0 (Timeline|Timeline_0 PlayFromStart)
      (:Update
        (for _array_element (Variables|Default|GetFlash)
          (Rendering|Material|SetScalarParameterValue _array_element "Intensity" _newtrack_0 :!class /Script/Engine.MaterialInstanceDynamic))))))

(event EventSpawnImpactEffect
  (params (HitLocation :type Vector :default "0, 0, 0") (OtherActorLocation :type Vector :default "0, 0, 0"))
  (bind _r (Variables|Hit|GetR))
  (bind _g (Variables|Hit|GetG))
  (bind _b (Variables|Hit|GetB))
  (bind _returnvalue (Niagara|SpawnSystematLocation "/Game/Particles/FX_HitEffect/FXS_HitEffect.FXS_HitEffect" (- (+ OtherActorLocation (* (Math|Vector|Normalize (- HitLocation OtherActorLocation)) (Variables|Hit|GetDistance))) "0, 0,10.000000") "0, 0, 0" "2.000000,2.000000,2.000000"))
  (Effects|Components|ParticleSystem|SetColorParameter _returnvalue "Color" (Math|Color|MakeColor _r _g _b (Variables|Hit|GetA)))
  (Effects|Components|ParticleSystem|SetFloatParameter _returnvalue "R" _r)
  (Effects|Components|ParticleSystem|SetFloatParameter _returnvalue "G" _g)
  (Effects|Components|ParticleSystem|SetFloatParameter _returnvalue "B" _b))

(fn ConstructionScript)

(fn UpdateLifeBar
  (bind _healthwidgetref (Variables|Default|GetHealthWidgetRef))
  (bind _healthcomponent (Variables|Default|GetHealthComponent))
  (Utilities|IsValid _healthcomponent
    (:Is%20Valid
      (bind _returnvalue (Class|HealthComponent|GetHealth _healthcomponent))
      (Utilities|IsValid _healthwidgetref
        (:Is%20Valid
          (Variables|/Game/UI/HealthLifeBars/W_EnemyHealthWithNumbers.W_EnemyHealthWithNumbers_C|SetHealth _healthwidgetref _returnvalue)
          (bind _returnvalue_2 (Class|HealthComponent|GetMaxHealth _healthcomponent))
          (Variables|/Game/UI/HealthLifeBars/W_EnemyHealthWithNumbers.W_EnemyHealthWithNumbers_C|SetMaxHealth _healthwidgetref _returnvalue_2)
          (Default|UpdateLifeText _healthwidgetref))))))

(fn SetMaterials
  (bind _returnvalue (Rendering|Material|CreateDynamicMaterialInstance (Variables|Character|GetMesh) 0 "/Game/Mannequin/Character/Materials/MI_Male_Body_Enemy.MI_Male_Body_Enemy" "None" :!class /Script/Engine.PrimitiveComponent))
  (bind _returnvalue_2 (Rendering|Material|CreateDynamicMaterialInstance (Variables|Character|GetMesh) 1 "/Game/Textures/Level1/Enemies/Razarac/Razarac_v3/MI_Razarac_Hood_v3.MI_Razarac_Hood_v3" "None" :!class /Script/Engine.PrimitiveComponent))
  (bind _returnvalue_3 (Rendering|Material|CreateDynamicMaterialInstance (Variables|Character|GetMesh) 2 "/Game/Textures/Level1/Enemies/Razarac/Razarac_v2/M_Razarac_HandShacklesTeethEyes_v2.M_Razarac_HandShacklesTeethEyes_v2" "None" :!class /Script/Engine.PrimitiveComponent))
  (bind _returnvalue_4 (Rendering|Material|CreateDynamicMaterialInstance (Variables|Character|GetMesh) 3 "/Game/Textures/Level1/Enemies/Razarac/Razarac_v3/MI_Razarac_CrystalShoulder_v3.MI_Razarac_CrystalShoulder_v3" "None" :!class /Script/Engine.PrimitiveComponent))
  (bind _returnvalue_5 (Rendering|Material|CreateDynamicMaterialInstance (Variables|Character|GetMesh) 4 "/Game/Textures/Level1/Enemies/Razarac/Razarac_v3/MI_Razarac_Body_v3.MI_Razarac_Body_v3" "None" :!class /Script/Engine.PrimitiveComponent))
  (Variables|Default|SetFlash (Utilities|Array|MakeArray _returnvalue_2 _returnvalue_3 _returnvalue_4 _returnvalue_5 _returnvalue)))