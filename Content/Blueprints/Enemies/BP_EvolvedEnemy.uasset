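; Evolved enemy Blueprint that handles health display, damage feedback and death for a pooled enemy.
; HealthComponent events refresh the health widget, while damage events play floating numbers from the damage widget's next text/animation slot plus a health-bar effect.
; Death drops rewards, sets the death animation flag, returns the actor to the pool after a delay, then notifies the GameMode.
; Impacts spawn a color-parameterized hit effect.
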(event ActorDeath(HealthComponent)
  ;[1 1 1] Actor Death
  (Class|DropRewardsComponent|DropRewards (Variables|Default|GetDropRewards))
  (Class|BasicEnemy|DeactivateforDeathAnim)
  (bind _asenemy_anim (Utilities|Casting|CastToEnemyAnim (Components|SkeletalMesh|GetAnimInstance (Variables|Character|GetMesh))))
  (Variables|/Game/Mannequin/Animations/Enemy/EnemyAnim.EnemyAnim_C|SetIsDead _asenemy_anim true)
  (Utilities|FlowControl|Delay 3.0)
  (Variables|/Game/Mannequin/Animations/Enemy/EnemyAnim.EnemyAnim_C|SetIsDead _asenemy_anim false)
  (Class|BasicEnemy|ReturntoPool)
  (bind _asw_enemy_health_with_numbers (Utilities|Casting|CastToW_EnemyHealthWithNumbers (UserInterface|GetUserWidgetObject (Variables|Default|GetHealthWidget))))
  (bind _output_get (Variables|Default|SetHealthWidgetRef _asw_enemy_health_with_numbers))
  (Default|UpdateLifeText _output_get)
  (bind _asbp_enemy_interface (Utilities|Casting|CastToBP_EnemyInterface (Game|GetGameMode)))
  (Default|DestroyEnemy _asbp_enemy_interface))

(event UpdateHealth(HealthComponent)
  (params (Health :type Float%20%28single-precision%29))
  (CallFunction|UpdateLifeBar))

(event OnComponentActivated(HealthComponent)
  (params (Component :type Actor%20Component%20Object%20Reference) (bReset :type Boolean)))

(event EventBeginPlay
  (bind _asw_enemy_health_with_numbers (Utilities|Casting|CastToW_EnemyHealthWithNumbers (UserInterface|GetUserWidgetObject (Variables|Default|GetHealthWidget))))
  (Variables|Default|SetHealthWidgetRef _asw_enemy_health_with_numbers)
  (CallFunction|UpdateLifeBar)
  (bind _asw_enemies_damage (Utilities|Casting|CastToW_EnemiesDamage (UserInterface|GetUserWidgetObject (Variables|Default|GetDamagePointsWidget))))
  (Variables|Default|SetDamagePointsWidgetRef _asw_enemies_damage))

(event Collision|EventActorBeginOverlap
  (params (OtherActor :type Actor%20Object%20Reference)))

(event EventSpawnImpactEffect
  (params (HitLocation :type Vector :default "0, 0, 0") (OtherActorLocation :type Vector :default "0, 0, 0"))
  (bind _r (Variables|HitEffect|GetR))
  (bind _g (Variables|HitEffect|GetG))
  (bind _b (Variables|HitEffect|GetB))
  (bind _returnvalue (Niagara|SpawnSystematLocation "/Game/Particles/FX_HitEffect/FXS_HitEffect.FXS_HitEffect" (- HitLocation "0, 0,10.000000") "0, 0, 0" "2.000000,2.000000,2.000000"))
  (Effects|Components|ParticleSystem|SetColorParameter _returnvalue "Color" (Math|Color|MakeColor _r _g _b (Variables|HitEffect|GetA)))
  (Effects|Components|ParticleSystem|SetFloatParameter _returnvalue "R" _r)
  (Effects|Components|ParticleSystem|SetFloatParameter _returnvalue "G" _g)
  (Effects|Components|ParticleSystem|SetFloatParameter _returnvalue "B" _b))

(event EventDrawDamageWidget
  (params (DamageReceived :type Float%20%28single-precision%29))
  (bind _damagepointswidgetref (Variables|Default|GetDamagePointsWidgetRef))
  (bind _healthwidgetref (Variables|Default|GetHealthWidgetRef))
  (bind (_text _anim) (Default|GetNextTextandAnim _damagepointswidgetref))
  (Rendering|Components|TextRender|SetText _text (Utilities|Text|ToText(Integer) (Math|Float|Truncate DamageReceived)))
  (UserInterface|Animation|PlayAnimation _damagepointswidgetref _anim 0.0 1 "Forward" 1.0 false)
  (UserInterface|Animation|PlayAnimation _healthwidgetref (Variables|/Game/UI/HealthLifeBars/W_EnemyHealthWithNumbers.W_EnemyHealthWithNumbers_C|GetDamageEffectAnim _healthwidgetref) 0.0 1 "Forward" 1.0 false))

(fn ConstructionScript)

(fn UpdateLifeBar
  (bind _healthwidgetref (Variables|Default|GetHealthWidgetRef))
  (bind _healthcomponent (Variables|Default|GetHealthComponent))
  (Utilities|IsValid _healthcomponent
    (:Is%20Valid
      (bind _returnvalue (Class|HealthComponent|GetHealth _healthcomponent))
      (Utilities|IsValid _healthwidgetref
        (:Is%20Valid
          (Variables|/Game/UI/HealthLifeBars/W_EnemyHealthWithNumbers.W_EnemyHealthWithNumbers_C|SetHealth _healthwidgetref _returnvalue)
          (bind _returnvalue_2 (Class|HealthComponent|GetMaxHealth _healthcomponent))
          (Variables|/Game/UI/HealthLifeBars/W_EnemyHealthWithNumbers.W_EnemyHealthWithNumbers_C|SetMaxHealth _healthwidgetref _returnvalue_2)
          (Default|UpdateLifeText _healthwidgetref))))))