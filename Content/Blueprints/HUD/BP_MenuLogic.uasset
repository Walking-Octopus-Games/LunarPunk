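; Menu navigation actor that manages focus and highlighting for an array of menu widgets, ticking even while paused.
; Direction events bound through BP_PlayerController cycle the focused index with wraparound on up/down and step SpinBox values on left/right.
; Tick lets mouse hover take keyboard focus, or keeps focus on a lone widget.
; Highlighting follows keyboard focus, tinting buttons and changing opacity on checkboxes and sliders.
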(event Custom|UpEvent
  ;[1 0.7551 0.2175] Directional Keys control
  (CallFunction|UpDownAction true))

(event Custom|RightEvent
  ;[1 0.7551 0.2175] Directional Keys control
  (CallFunction|RightLeftAction true))

(event Custom|LeftEvent
  ;[1 0.7551 0.2175] Directional Keys control
  (CallFunction|RightLeftAction false))

(event Custom|DownEvent
  ;[1 0.7551 0.2175] Directional Keys control
  (CallFunction|UpDownAction false))

(event EventBeginPlay
  ;[1 0.7551 0.2175] Directional Keys control
  (bind _asbp_player_controller (Utilities|Casting|CastToBP_PlayerController (Game|GetPlayerController 0)))
  (Class|Actor|SetTickablewhenPaused true)
  (EventDispatchers|AssignUpEvent _asbp_player_controller (delegate Custom|UpEvent))
  (EventDispatchers|BindEventtoDownEvent _asbp_player_controller (delegate Custom|DownEvent))
  (EventDispatchers|AssignRightEvent _asbp_player_controller (delegate Custom|RightEvent))
  (EventDispatchers|AssignLeftEvent _asbp_player_controller (delegate Custom|LeftEvent)))

(event EventTick
  (params (DeltaSeconds :type Float%20%28single-precision%29))
  (if (> (Utilities|Array|Length (Variables|Default|GetWidgetsArray)) 1)
    (CallFunction|ChangeFocus false)
    (for (_array_element _array_index) (Variables|Default|GetWidgetsArray)
      ;[0.4316 1 0.8694] Change Focus on mouse Hover
      (Utilities|IsValid _array_element
        (:Is%20Valid
          (if (Widget|IsHovered _array_element)
            (Variables|Default|SetFocusedButton _array_index)
            (Widget|SetKeyboardFocus _array_element)
            (CallFunction|ChangeFocus true)))))
    (else
      ;[1 1 1] If there is only 1 widget, don't change the focus.
      (if (> (Utilities|Array|Length (Variables|Default|GetWidgetsArray)) 0)
        (Variables|Default|SetFocusedButton 0)
        (Widget|SetKeyboardFocus (Utilities|Array|Get(acopy) (Variables|Default|GetWidgetsArray)))
        (CallFunction|ChangeFocus true)))))

(fn ConstructionScript)

(fn ChangeFocus
  (params (IsFocused :type Boolean))
  (for _array_element (Variables|Default|GetWidgetsArray)
    (if (Class|Widget|HasKeyboardFocus _array_element)
      (CallFunction|ApplyHighlightEffect _array_element)
      (else
        (CallFunction|RemoveHighlightEffect _array_element)))))

(fn UpDownAction
  (params (Up/Down :type Boolean))
  (bind _widgetsarray (Variables|Default|GetWidgetsArray))
  (bind _returnvalue (Utilities|Array|Length _widgetsarray))
  (if Up/Down
    (bind _result (Math|Integer|DecrementInt (+ (Variables|Default|GetFocusedButton) _returnvalue))
      (:%20%20
        (Variables|Default|SetFocusedButton (Math|Integer|%(Integer) _result _returnvalue))))
    (else
      (bind _result_2 (Math|Integer|IncrementInt (+ (Variables|Default|GetFocusedButton) _returnvalue))
        (:%20%20
          (Variables|Default|SetFocusedButton (Math|Integer|%(Integer) _result_2 _returnvalue))))))
  (bind _asw_menu_button (Utilities|Casting|CastToW_MenuButton (Utilities|Array|Get(acopy) (Variables|Default|GetWidgetsArray) (Variables|Default|GetFocusedButton))))
  (Widget|SetKeyboardFocus (Variables|/Game/UI/W_MenuButton.W_MenuButton_C|GetMenuButton _asw_menu_button)))

(fn InitialFocusedButtonSet
  (bind _output_get (Variables|Default|SetFocusedButton 0))
  (if (Utilities|IsValid (Utilities|Array|Get(acopy) (Variables|Default|GetWidgetsArray) _output_get))
    (bind _asw_menu_button (Utilities|Casting|CastToW_MenuButton (Utilities|Array|Get(acopy) (Variables|Default|GetWidgetsArray) _output_get))
      (:then
        (Widget|SetKeyboardFocus (Variables|/Game/UI/W_MenuButton.W_MenuButton_C|GetMenuButton _asw_menu_button))
        (CallFunction|ChangeFocus true))
      (:CastFailed
        (bind _asw_menu_checkbox (Utilities|Casting|CastToW_MenuCheckbox (Utilities|Array|Get(acopy) (Variables|Default|GetWidgetsArray) _output_get))
          (:then
            (Widget|SetKeyboardFocus (Variables|/Game/UI/W_MenuCheckbox.W_MenuCheckbox_C|GetCheckBox _asw_menu_checkbox))
            (CallFunction|ChangeFocus true))
          (:CastFailed
            (bind _asw_menu_slider (Utilities|Casting|CastToW_MenuSlider (Utilities|Array|Get(acopy) (Variables|Default|GetWidgetsArray) _output_get)))
            (Widget|SetKeyboardFocus (Variables|/Game/UI/W_MenuSlider.W_MenuSlider_C|GetVariableSlider _asw_menu_slider))
            (CallFunction|ChangeFocus true)))))))

(fn RightLeftAction
  (params (Right/Left :type Boolean))
  (bind _asspin_box (Utilities|Casting|CastToSpinBox (Utilities|Array|Get(acopy) (Variables|Default|GetWidgetsArray) (Variables|Default|GetFocusedButton))))
  (if Right/Left
    (bind _result (Math|Float|IncrementFloat (Class|SpinBox|GetValue _asspin_box))
      (:%20%20
        (Class|SpinBox|SetValue _asspin_box _result)))
    (else
      (bind _result_2 (Math|Float|DecrementFloat (Class|SpinBox|GetValue _asspin_box))
        (:%20%20
          (Class|SpinBox|SetValue _asspin_box _result_2))))))

(fn ApplyHighlightEffect
  (params (Widget :type Widget%20Object%20Reference))
  (Utilities|FlowControl|Sequence
    (:then_0
      (bind _asbutton (Utilities|Casting|CastToButton Widget))
      (Class|Button|SetBackgroundColor _asbutton "(R=0.416174,G=0.084765,B=0.489583,A=1.000000)"))
    (:then_1
      (bind _ascheck_box (Utilities|Casting|CastToCheckBox Widget))
      (Widget|SetRenderOpacity _ascheck_box 1.0))
    (:then_2
      (bind _asslider (Utilities|Casting|CastToSlider Widget))
      (Widget|SetRenderOpacity _asslider 1.0))))

(fn RemoveHighlightEffect
  (params (NewParam :type Widget%20Object%20Reference))
  (Utilities|FlowControl|Sequence
    (:then_0
      (bind _asbutton (Utilities|Casting|CastToButton NewParam))
      (Class|Button|SetBackgroundColor _asbutton "(R=1.000000,G=1.000000,B=1.000000,A=1.000000)"))
    (:then_1
      (bind _ascheck_box (Utilities|Casting|CastToCheckBox NewParam))
      (Widget|SetRenderOpacity _ascheck_box 0.4))
    (:then_2
      (bind _asslider (Utilities|Casting|CastToSlider NewParam))
      (Widget|SetRenderOpacity _asslider 0.4))))