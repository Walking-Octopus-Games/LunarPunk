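; Player character Blueprint that links health, abilities, HUD, game mode and animation.
; Health events drive a timeline hit flash on dynamic body materials and, on death, the AnimBP and game mode; Pause input calls the game mode.
; It pushes initial health and portal-destroy availability to the HUD.
; Also handles gated debug-drawn grenade arc prediction, a timed throw flag, and red/green turret placement tinting from collider overlaps.
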(event ActorDeath(HealthComponent)
  (bind _asiska_anim_bp (Utilities|Casting|CastToIska_AnimBP (Components|SkeletalMesh|GetAnimInstance (Variables|Character|GetMesh))))
  (Variables|/Game/Mannequin/Animations/Iska_AnimBP.Iska_AnimBP_C|SetIsDead _asiska_anim_bp true)
  (bind _asbp_lunar_punk_game_mode (Utilities|Casting|CastToBP_LunarPunkGameMode (Game|GetGameMode)))
  (Default|PlayerDeath _asbp_lunar_punk_game_mode))

(event OnComponentBeginOverlap(PositioningCollider)
  (params (OverlappedComponent :type Primitive%20Component%20Object%20Reference) (OtherActor :type Actor%20Object%20Reference) (OtherComp :type Primitive%20Component%20Object%20Reference) (OtherBodyIndex :type Integer) (bFromSweep :type Boolean) (SweepResult :type Hit%20Result%20Structure%20%28by%20ref%29))
  (Rendering|Material|SetVectorParameterValue (Variables|Default|GetTurretPositioningMaterial) "Color" "(R=1.000000,G=0.050000,B=0.050000,A=1.000000)" :!class /Script/Engine.MaterialInstanceDynamic))

(event OnComponentEndOverlap(PositioningCollider)
  (params (OverlappedComponent :type Primitive%20Component%20Object%20Reference) (OtherActor :type Actor%20Object%20Reference) (OtherComp :type Primitive%20Component%20Object%20Reference) (OtherBodyIndex :type Integer))
  (if (== (Utilities|Array|Length (Collision|GetOverlappingActors (Variables|Default|GetPositioningCollider) 0 :!class /Script/Engine.PrimitiveComponent)) 0)
    (Rendering|Material|SetVectorParameterValue (Variables|Default|GetTurretPositioningMaterial) "Color" "(R=0.000000,G=1.000000,B=0.000000,A=1.000000)" :!class /Script/Engine.MaterialInstanceDynamic)))

(event DamageReceived(HealthComponent)
  (params (Damage :type Float%20%28single-precision%29))
  (CallFunction|EffectwhenHitted))

(event Custom|EffectWhenHitted
  (bind _newtrack_0 (Timeline|Timeline_0 PlayFromStart)
    (:Update
      (for _array_element (Variables|Default|GetFlash)
        (Rendering|Material|SetScalarParameterValue _array_element "Intensity" _newtrack_0 :!class /Script/Engine.MaterialInstanceDynamic)))))

(event Custom|SetAvailableToDestroyPortal_Event_0
  (params (Available :type Boolean) (maxTime :type Float%20%28single-precision%29))
  (bind _asbp_hud (Utilities|Casting|CastToBP_HUD (HUD|GetHUD (Game|GetPlayerController 0))))
  (Default|SetAvilabletoDestroyPortal (Variables|/Game/Blueprints/HUD/BP_HUD.BP_HUD_C|GetHUDPlayerCharacter _asbp_hud) Available maxTime))

(event EventBeginPlay
  (bind _healthcomponent (Variables|Default|GetHealthComponent))
  ;[1 1 1] Init player health in HUD
  (CallFunction|SetMaterials)
  (bind _returnvalue (Class|HealthComponent|GetActualHealth _healthcomponent))
  (bind _returnvalue_2 (Class|HealthComponent|GetMaxHealth _healthcomponent))
  (bind _asbp_hud (Utilities|Casting|CastToBP_HUD (HUD|GetHUD (Game|GetPlayerController 0))))
  (Utilities|IsValid (Variables|/Game/Blueprints/HUD/BP_HUD.BP_HUD_C|GetHUDPlayerCharacter _asbp_hud)
    (:Is%20Valid
      (Default|SetHealthPlayer (Variables|/Game/Blueprints/HUD/BP_HUD.BP_HUD_C|GetHUDPlayerCharacter _asbp_hud) (/ _returnvalue _returnvalue_2))
      (EventDispatchers|BindEventtoSetAvailabletoDestroyPortal (Variables|Default|GetDestroyPortalAbilityComponent) (delegate Custom|SetAvailableToDestroyPortal_Event_0)))))

(event EventTick
  (params (DeltaSeconds :type Float%20%28single-precision%29)))

(event EventShowGranadePath
  (bind _startshootreferencepoint (Variables|Default|GetStartShootReferencePoint))
  (bind _returnvalue (Transformation|GetSocketTransform _startshootreferencepoint "None" "RTS_World"))
  (Utilities|FlowControl|Gate true ; enters at Open
    (:Exit
      (Class|GameplayStatics|BlueprintPredictProjectilePathbyTraceChannel (.location _returnvalue) (* (Math|Vector|GetForwardVector (.rotation _returnvalue)) (* (Variables|/Script/Lunarpunk.GranadeAbilityComponent|GetGranadeDistance (Variables|Default|GetGrenadeAbilityComponent)) 5e+02)) false 1e+01 "ECC_Visibility" false (Utilities|Array|MakeArray self) "ForDuration"))))

(event EventHideGranadePath
  (bind _startshootreferencepoint (Variables|Default|GetStartShootReferencePoint))
  (bind _returnvalue (Transformation|GetSocketTransform _startshootreferencepoint "None" "RTS_World"))
  (Utilities|FlowControl|Gate true ; enters at Close
    (:Exit
      (Class|GameplayStatics|BlueprintPredictProjectilePathbyTraceChannel (.location _returnvalue) (* (Math|Vector|GetForwardVector (.rotation _returnvalue)) (* (Variables|/Script/Lunarpunk.GranadeAbilityComponent|GetGranadeDistance (Variables|Default|GetGrenadeAbilityComponent)) 5e+02)) false 1e+01 "ECC_Visibility" false (Utilities|Array|MakeArray self) "ForDuration"))))

(event EventThrowGrenadeAnimation
  (Variables|Default|SetIs%20Throwing%20Grenade true)
  (Utilities|FlowControl|Delay 0.4)
  (Variables|Default|SetIs%20Throwing%20Grenade false))

(event Input|ActionEvents|InputActionPause
  (params (Key :type Key%20Structure :default "None"))
  (:Pressed
    (bind _asbp_lunar_punk_game_mode (Utilities|Casting|CastToBP_LunarPunkGameMode (Game|GetGameMode)))
    (Default|PauseGame _asbp_lunar_punk_game_mode)))

(fn ConstructionScript
  (Variables|Default|SetStartShootReferencePoint (Variables|Default|GetHitscanShootReference))
  (bind _returnvalue (Rendering|Material|CreateDynamicMaterialInstance (Variables|Default|GetTurretPositioningIndicator) :!class /Script/Engine.DecalComponent))
  (Variables|Default|SetTurretPositioningMaterial _returnvalue))

(fn SetMaterials
  (bind _returnvalue (Rendering|Material|CreateDynamicMaterialInstance (Variables|Character|GetMesh) 0 "/Game/Textures/Level1/Character/M_CharacterLegs.M_CharacterLegs" "None" :!class /Script/Engine.PrimitiveComponent))
  (bind _returnvalue_2 (Rendering|Material|CreateDynamicMaterialInstance (Variables|Character|GetMesh) 2 "/Game/Textures/Level1/Character/M_CharacterHead.M_CharacterHead" "None" :!class /Script/Engine.PrimitiveComponent))
  (bind _returnvalue_3 (Rendering|Material|CreateDynamicMaterialInstance (Variables|Character|GetMesh) 3 "/Game/Textures/Level1/Character/M_CharacterMask.M_CharacterMask" "None" :!class /Script/Engine.PrimitiveComponent))
  (bind _returnvalue_4 (Rendering|Material|CreateDynamicMaterialInstance (Variables|Character|GetMesh) 1 "/Game/Textures/Level1/Character/M_CharacterBody.M_CharacterBody" "None" :!class /Script/Engine.PrimitiveComponent))
  (Variables|Default|SetFlash (Utilities|Array|MakeArray _returnvalue _returnvalue_2 _returnvalue_3 _returnvalue_4)))