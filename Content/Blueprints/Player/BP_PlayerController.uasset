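; Player controller that turns gamepad and keyboard input into directional and back events for menus, plus right-stick events for turret and upgrade selection.
; Tick decodes the RawInput D-pad axis by tolerance and debounces D-pad and DualSense stick to fire once per push.
; Raw polling stays off until the axis first reads its idle value.
; Xbox D-pad and arrow keys call the same directional events directly.
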(event EventBeginPlay)

(event EventTick
  (params (DeltaSeconds :type Float%20%28single-precision%29))
  (bind _returnvalue (Class|Actor|GetInputAxisKeyValue))
  (bind _returnvalue_2 (Class|Actor|GetInputAxisKeyValue))
  (bind _returnvalue_3 (Input|AxisValues|GetRawDirectionalPad))
  (bind _returnvalue_4 (<= _returnvalue -0.75))
  (bind _returnvalue_5 (>= _returnvalue_2 0.75))
  (bind _returnvalue_6 (Math|Float|NearlyEqual(Float) _returnvalue_3 1.14 0.1))
  ;[1 1 1] Mapping for RAWInput Directional Pad (Menu)
  (if (Variables|Default|GetIsEnabledRawController)
    (Utilities|FlowControl|Sequence
      (:then_0
        (if (Math|Float|NearlyEqual(Float) _returnvalue_3 0.0 0.1)
          (if (!= (Variables|Default|GetLastInput) 1)
            (Default|CallUpEvent)
            (Class|LunarPunkPlayerController|UpDirectionalPad)
            (Variables|Default|SetLastInput 1))))
      (:then_1
        (if (Math|Float|NearlyEqual(Float) _returnvalue_3 0.285714 0.1)
          (if (!= (Variables|Default|GetLastInput) 2)
            (Default|CallRightEvent)
            (Class|LunarPunkPlayerController|RightDirectionalPad)
            (Variables|Default|SetLastInput 2))))
      (:then_2
        (if (Math|Float|NearlyEqual(Float) _returnvalue_3 0.571429 0.1)
          (if (!= (Variables|Default|GetLastInput) 3)
            (Default|CallDownEvent)
            (Class|LunarPunkPlayerController|DownDirectionalPad)
            (Variables|Default|SetLastInput 3))))
      (:then_3
        (if (Math|Float|NearlyEqual(Float) _returnvalue_3 0.857143 0.1)
          (if (!= (Variables|Default|GetLastInput) 4)
            (Default|CallLeftEvent)
            (Class|LunarPunkPlayerController|LeftDirectionalPad)
            (Variables|Default|SetLastInput 4))))
      (:then_4
        (if _returnvalue_6
          ;;[1 1 1] Set Idle input as 0
          (Variables|Default|SetLastInput 0 :!label _label)))
      (:then_5
        (Utilities|FlowControl|Sequence
          (:then_0
            ;[1 1 1] Mapping DualSense Right Thumbstick for Turret and Upgrade Selection
            (if _returnvalue_4
              (if (not (Variables|Default|GetLastRightThumbstickLeftResult))
                (Default|CallRightThumbStickLeft)
                (Variables|Default|SetLastRightThumbstickLeftResult true))
              (else
                (Variables|Default|SetLastRightThumbstickLeftResult _returnvalue_4))))
          (:then_1
            (if _returnvalue_5
              (if (not (Variables|Default|GetLastRightThumbstickRightResult))
                (Default|CallRightThumbStickRight)
                (Variables|Default|SetLastRightThumbstickRightResult true))
              (else
                (Variables|Default|SetLastRightThumbstickRightResult _returnvalue_5)))))))
    (else
      (Variables|Default|SetIsEnabledRawController _returnvalue_6)
      (goto _label))))

(event Input|GamepadEvents|GamepadFaceButtonRight
  (params (Key :type Key%20Structure :default "None"))
  ;[1 1 1] Mapping Back  on Menu
  (:Pressed
    (Default|CallBackEvent)))

(event Input|GamepadEvents|GamepadDPadUp
  (params (Key :type Key%20Structure :default "None"))
  ;[0.3166 1 0.4028] Mapping for Gamepad (Xbox) and Keyboard
  (:Pressed
    (Default|CallUpEvent)))

(event Input|KeyboardEvents|Up
  (params (Key :type Key%20Structure :default "None"))
  ;[0.3166 1 0.4028] Mapping for Gamepad (Xbox) and Keyboard
  (:Pressed
    (Default|CallUpEvent)))

(event Input|GamepadEvents|GamepadDPadDown
  (params (Key :type Key%20Structure :default "None"))
  ;[0.3166 1 0.4028] Mapping for Gamepad (Xbox) and Keyboard
  (:Pressed
    (Default|CallDownEvent)))

(event Input|KeyboardEvents|Down
  (params (Key :type Key%20Structure :default "None"))
  ;[0.3166 1 0.4028] Mapping for Gamepad (Xbox) and Keyboard
  (:Pressed
    (Default|CallDownEvent)))

(event Input|KeyboardEvents|Right
  (params (Key :type Key%20Structure :default "None"))
  ;[0.3166 1 0.4028] Mapping for Gamepad (Xbox) and Keyboard
  (:Pressed
    (Default|CallRightEvent)))

(event Input|GamepadEvents|GamepadDPadRight
  (params (Key :type Key%20Structure :default "None"))
  ;[0.3166 1 0.4028] Mapping for Gamepad (Xbox) and Keyboard
  (:Pressed
    (Default|CallRightEvent)))

(event Input|GamepadEvents|GamepadDPadLeft
  (params (Key :type Key%20Structure :default "None"))
  ;[0.3166 1 0.4028] Mapping for Gamepad (Xbox) and Keyboard
  (:Pressed
    (Default|CallLeftEvent)))

(event Input|KeyboardEvents|Left
  (params (Key :type Key%20Structure :default "None"))
  ;[0.3166 1 0.4028] Mapping for Gamepad (Xbox) and Keyboard
  (:Pressed
    (Default|CallLeftEvent)))

(fn ConstructionScript)