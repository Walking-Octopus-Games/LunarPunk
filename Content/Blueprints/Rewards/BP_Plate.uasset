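; Plate reward actor that blinks near the end of its lifetime and shows its quantity in a widget.
; Tick drives the blink by swapping the cylinder material to M_None briefly, then waiting between blinks.
; GotoHUD plays a screen animation of the plate icon and amount flying to the HUD, then calls AddToHUD once it finishes.
; GetTypeOfReward identifies the reward by its own class.
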(event EventBeginPlay)

(event Collision|EventActorBeginOverlap
  (params (OtherActor :type Actor%20Object%20Reference)))

(event EventTick
  (params (DeltaSeconds :type Float%20%28single-precision%29))
  (if (>= (Variables|Default|GetCurrentTime) (- (Variables|Default|GetLifetime) (Variables|Default|GetTimeToLastToStartBlinking)))
    (if (Variables|Default|GetIsVanished)
      (Variables|Default|SetCurrentTimeBetweenBlinks (+ (Variables|Default|GetCurrentTimeBetweenBlinks) (Utilities|Time|GetWorldDeltaSeconds)))
      (if (>= (Variables|Default|GetCurrentTimeBetweenBlinks) (Variables|Default|GetTimeToNextBlink))
        (Variables|Default|SetIsVanished false))
      (else
        (Variables|Default|SetCurrentTimeBetweenBlinks 0.0)
        (Variables|Default|SetIsVanished true)
        (Rendering|Material|SetMaterial (Variables|Default|GetCylinder) 0 "/Game/Materials/M_None.M_None")
        (Utilities|FlowControl|Delay (Variables|Default|GetTimeIsDisapeared))
        (Rendering|Material|SetMaterial (Variables|Default|GetCylinder) 0 "/Game/Materials/Plates/MI_Plate.MI_Plate")))))

(event EventGotoHUD
  (params (QuantityToAdd :type Integer))
  (bind _returnvalue (UserInterface|CreateWidget (Variables|Default|GetGoToHUDWidget) (Game|GetPlayerController 0)))
  (bind _asw_reward_going_to_hud (Utilities|Casting|CastToW_RewardGoingToHUD _returnvalue)
    (:then
      (Default|SetPlatesIcon _asw_reward_going_to_hud)
      (UserInterface|Viewport|AddtoViewport _asw_reward_going_to_hud 0)
      (Rendering|Components|TextRender|SetText (Variables|/Game/UI/HUD_Effects/W_RewardGoingToHUD.W_RewardGoingToHUD_C|GetNumPlates _asw_reward_going_to_hud) (Utilities|Text|ToText(String) (Utilities|String|Append "x" (Utilities|String|ToString(Text) (Utilities|Text|ToText(Integer) QuantityToAdd)))))
      (UserInterface|Animation|PlayAnimation _asw_reward_going_to_hud (Variables|/Game/UI/HUD_Effects/W_RewardGoingToHUD.W_RewardGoingToHUD_C|GetGoToPlates _asw_reward_going_to_hud) 0.0 1 "Forward" 1.0 false)
      (Utilities|FlowControl|Delay (Class|WidgetAnimation|GetEndTime (Variables|/Game/UI/HUD_Effects/W_RewardGoingToHUD.W_RewardGoingToHUD_C|GetGoToPlates _asw_reward_going_to_hud))))
    (:CastFailed
      _))
  (Class|Reward|AddtoHUD QuantityToAdd))

(event EventUpdateQuantityWidget
  (bind _asw_plates_widget (Utilities|Casting|CastToW_PlatesWidget (UserInterface|GetUserWidgetObject (Variables|Default|GetPlatesWidget))))
  (Rendering|Components|TextRender|SetText (Variables|/Game/UI/HUD_Effects/W_PlatesWidget.W_PlatesWidget_C|GetPlatesNum _asw_plates_widget) (Utilities|Text|ToText(Integer) (Variables|Default|GetQuantity))))

(fn ConstructionScript)

(fn GetTypeOfReward
  (return (Utilities|GetClass self)))