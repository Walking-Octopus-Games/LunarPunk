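; BP_Sector is a level sector actor with a floor whose material can be swapped and a wall that can be raised.
; ChangeMaterial applies an indexed entry from the Materials array to the floor.
; UpWall enables the invisible wall's collision, disables the Collision and Exit components' collision, then lifts the visible wall from its current height using the Up timeline scaled by High.
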(event EventBeginPlay)

(event Collision|EventActorBeginOverlap
  (params (OtherActor :type Actor%20Object%20Reference)))

(event EventTick
  (params (DeltaSeconds :type Float%20%28single-precision%29)))

(event EventChangeMaterial
  (params (MaterialIndex :type Integer))
  (Rendering|Material|SetMaterial (Variables|Default|GetFloor) 0 (Utilities|Array|Get(acopy) (Variables|Default|GetMaterials) MaterialIndex)))

(event EventUpWall
  (bind _wall (Variables|Default|GetWall))
  (bind _returnvalue (Transformation|GetWorldLocation _wall))
  (Collision|SetCollisionEnabled (Variables|Default|GetInvisibleWall) "QueryAndPhysics")
  (Collision|SetCollisionEnabled (Variables|Default|GetCollision) "NoCollision")
  (Collision|SetCollisionEnabled (Variables|Default|GetExit) "NoCollision")
  (bind _output_get (Variables|Default|SetInitialHigh (.z _returnvalue)))
  (bind _newtrack_0 (Timeline|Up Play)
    (:Update
      (Transformation|SetWorldLocation _wall (Math|Vector|MakeVector (.x _returnvalue) (.y _returnvalue) (+ _output_get (* (Variables|Default|GetHigh) _newtrack_0))) false false))))

(fn ConstructionScript)