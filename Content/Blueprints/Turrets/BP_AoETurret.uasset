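; BP_AoETurret is an area-of-effect turret actor with health and an overhead-style health display; its graph holds no attack logic.
; On BeginPlay it points its VampirismComponent at the player character's HealthComponent as the one to restore, then caches its W_EnemyHealth widget.
; It copies current and max health into that widget at startup and whenever the HealthComponent fires PlayerBeingDamage.
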(event PlayerBeingDamage(HealthComponent)
  (bind _healthwidgetref (Variables|Default|GetHealthWidgetRef))
  (bind _healthcomponent (Variables|Default|GetHealthComponent))
  (bind _returnvalue (Class|HealthComponent|GetHealth _healthcomponent))
  (Variables|/Game/UI/W_EnemyHealth.W_EnemyHealth_C|SetHealth _healthwidgetref _returnvalue)
  (bind _returnvalue_2 (Class|HealthComponent|GetMaxHealth _healthcomponent))
  (Variables|/Game/UI/W_EnemyHealth.W_EnemyHealth_C|SetMaxHealth _healthwidgetref _returnvalue_2))

(event EventBeginPlay
  (bind _healthcomponent (Variables|Default|GetHealthComponent))
  (bind _asbp_player_character (Utilities|Casting|CastToBP_PlayerCharacter (Game|GetPlayerCharacter 0)))
  (Variables|/Script/HexBusters.VampirismComponent|SetHealthComponentToRestore (Variables|Default|GetVampirismComponent) (Variables|/Script/HexBusters.PlayableCharacter|GetHealthComponent _asbp_player_character))
  (bind _asw_enemy_health (Utilities|Casting|CastToW_EnemyHealth (UserInterface|GetUserWidgetObject (Variables|Default|GetHealthWidget))))
  (Variables|Default|SetHealthWidgetRef _asw_enemy_health)
  (bind _returnvalue (Class|HealthComponent|GetHealth _healthcomponent))
  (Variables|/Game/UI/W_EnemyHealth.W_EnemyHealth_C|SetHealth (Variables|Default|GetHealthWidgetRef) _returnvalue)
  (bind _returnvalue_2 (Class|HealthComponent|GetMaxHealth _healthcomponent))
  (Variables|/Game/UI/W_EnemyHealth.W_EnemyHealth_C|SetMaxHealth (Variables|Default|GetHealthWidgetRef) _returnvalue_2))

(fn ConstructionScript)