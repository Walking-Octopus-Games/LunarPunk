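; Turret helper component that manages an on-screen icon indicating the position of its owning turret.
; InitializeWidget creates a W_TurretPositionHelperIcon, selects its image from the owner's turret class, and adds it to the viewport hidden.
; Events show or hide the icon, set its viewport position and rotation from supplied values, and forward damage, death and reactivation effects to the widget.
; The damage effect plays only while ShowingIconInHUD is set.
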(event EventBeginPlay)

(event EventTick
  (params (DeltaSeconds :type Float%20%28single-precision%29)))

(event EventShowIconinHUD
  (bind _iconwidget (Variables|Default|GetIconWidget))
  (Utilities|IsValid _iconwidget
    (:Is%20Valid
      (Widget|SetVisibility _iconwidget "Visible"))))

(event EventUpdateIconPositioninHUD
  (params (HUDPosition :type Vector%202D%20Structure%20%28by%20ref%29) (AngleRotation :type Float%20%28single-precision%29))
  (bind _iconwidget (Variables|Default|GetIconWidget))
  (Utilities|IsValid _iconwidget
    (:Is%20Valid
      (Class|UserWidget|SetPositioninViewport _iconwidget HUDPosition true)
      (Default|RotateIconBox (Variables|Default|GetIconWidget) AngleRotation))))

(event EventRemoveIconinHUD
  (bind _iconwidget (Variables|Default|GetIconWidget))
  (Utilities|IsValid _iconwidget
    (:Is%20Valid
      (Widget|SetVisibility _iconwidget "Hidden"))))

(event EventShowDamageEffect
  (params (Damage :type Float%20%28single-precision%29))
  (bind _iconwidget (Variables|Default|GetIconWidget))
  (if (Variables|Default|GetbShowingIconInHUD)
    (Utilities|IsValid _iconwidget
      (:Is%20Valid
        (Default|DamageEffect _iconwidget)))))

(event EventShowDeathEffect
  (bind _iconwidget (Variables|Default|GetIconWidget))
  (Utilities|IsValid _iconwidget
    (:Is%20Valid
      (Default|DeathEffect _iconwidget))))

(event EventInitializeWidget
  (bind _returnvalue (UserInterface|CreateWidget "/Game/UI/HUD_Effects/W_TurretPositionHelperIcon.W_TurretPositionHelperIcon_C"))
  (bind _output_get (Variables|Default|SetIconWidget _returnvalue))
  (bind _asturret (Utilities|Casting|CastToTurretClass (Utilities|GetClass (Components|GetOwner))))
  (Default|SelectImage _output_get _asturret)
  (Widget|SetVisibility _output_get "Hidden")
  (UserInterface|Viewport|AddtoViewport _output_get 0))

(event EventShowReactivatedEffect
  (bind _iconwidget (Variables|Default|GetIconWidget))
  (Utilities|IsValid _iconwidget
    (:Is%20Valid
      (Default|ReactivatedEffect _iconwidget))))