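; Projectile turret Blueprint that drives the turret's world UI: health, info and repair progress widgets.
; BeginPlay caches the widgets and binds repair and upgrade events, with the progress ring timed for either repair or revive.
; Health changes refresh the health display and choose action prompts from health and the player's plates versus repair cost.
; Damage plays a widget animation, and draw/remove events set info panel opacity, dimming it while moving.
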(event DamageReceived(HealthComponent)
  (params (Damage :type Float%20%28single-precision%29))
  (bind _healthwidget (Variables|Default|GetHealthWidget))
  (Utilities|IsValid _healthwidget
    (:Is%20Valid
      (bind _asw_turrets_health (Utilities|Casting|CastToW_TurretsHealth (UserInterface|GetWidget _healthwidget)))
      (UserInterface|Animation|PlayAnimation _asw_turrets_health (Variables|/Game/UI/HealthLifeBars/W_TurretsHealth.W_TurretsHealth_C|GetDamageEffectAnim _asw_turrets_health) 0.0 1 "Forward" 1.0 false))))

(event UpdateHealth(HealthComponent)
  (params (Health :type Float%20%28single-precision%29))
  (CallFunction|UpdateHealthWidget)
  (bind _aslunar_punk_game_mode (Utilities|Casting|CastToLunarPunkGameMode (Game|GetGameMode)))
  (Utilities|IsValid (Class|LunarPunkGameMode|GetPlatesManager _aslunar_punk_game_mode)
    (:Is%20Valid
      (Class|Turret|RefreshInfoWidget (Class|PlatesManager|GetCurrentPlates (Class|LunarPunkGameMode|GetPlatesManager _aslunar_punk_game_mode))))))

(event Custom|Repairing_Event
  ;[1 1 1] RepairingEvent to Update widget
  (bind _returnvalue (Class|HealthComponent|GetActualHealth (Variables|Default|GetHealthComponent)))
  (if (> _returnvalue 0.0)
    (Default|SetProgress (Variables|Default|GetRepairWidgetRef) (/ (Variables|Default|GetCurrentTimeLeftToHeal) (Variables|Default|GetMaxTimeLeftToRepair)))
    (else
      (Default|SetProgress (Variables|Default|GetRepairWidgetRef) (/ (Variables|Default|GetCurrentTimeLeftToHeal) (Variables|Default|GetMaxTimeLeftToRevive))))))

(event Custom|StopRepairingEvent
  (Default|SetProgress (Variables|Default|GetRepairWidgetRef) 0.0))

(event Custom|UpgradeInfo
  (params (UpgradesInfo :type Upgrades%20Info%20Structure))
  (Default|UpdateUpgradesInfo (Variables|Default|GetInfoTurretRef) UpgradesInfo))

(event EventBeginPlay
  (bind _asw_turrets_health (Utilities|Casting|CastToW_TurretsHealth (UserInterface|GetUserWidgetObject (Variables|Default|GetHealthWidget))))
  (Variables|Default|SetHealthWidgetRef _asw_turrets_health)
  (bind _asw_info_turret (Utilities|Casting|CastToW_InfoTurret (UserInterface|GetUserWidgetObject (Variables|Default|GetInfoWidget)))
    (:then
      (Utilities|IsValid _asw_info_turret
        (:Is%20Valid
          (bind _output_get (Variables|Default|SetInfoTurretRef _asw_info_turret))
          (Default|SetType _output_get (Utilities|GetClass self))
          (Widget|Transform|SetRenderScale _output_get "(X=0.600000,Y=0.600000)")
          (Class|Turret|RefreshInfoWidget))
        (:Is%20Not%20Valid
          _)))
    (:CastFailed
      _))
  (CallFunction|UpdateHealthWidget)
  (bind _ascircular_progress_bar_widget (Utilities|Casting|CastToCircularProgressBarWidget (UserInterface|GetUserWidgetObject (Variables|Default|GetRepairWidget))))
  (Variables|Default|SetRepairWidgetRef _ascircular_progress_bar_widget)
  (EventDispatchers|AssignRepairing (delegate Custom|Repairing_Event))
  (EventDispatchers|BindEventtoStopRepairing (delegate Custom|StopRepairingEvent))
  (EventDispatchers|BindEventtoUpdateUpgradesInfoEvent (delegate Custom|UpgradeInfo)))

(event EventTick
  (params (DeltaSeconds :type Float%20%28single-precision%29)))

(event EventDrawInfoWidget
  (bind _infowidget (Variables|Default|GetInfoWidget))
  (bind _infoturretref (Variables|Default|GetInfoTurretRef))
  (bind _returnvalue (UserInterface|GetUserWidgetObject _infowidget))
  (bind _actionstext (Variables|/Game/UI/HUD_Effects/W_InfoTurret.W_InfoTurret_C|GetActionsText _infoturretref))
  (Utilities|IsValid _returnvalue
    (:Is%20Valid
      (bind _returnvalue_2 (Class|Turret|GetState))
      (if (Utilities|Enum|Equal(Enum) _returnvalue_2 "Moving")
        (Widget|SetRenderOpacity _returnvalue 0.3)
        (Default|ShowActionKey (Variables|Default|GetInfoTurretRef) "NewEnumerator3")
        (Widget|SetRenderOpacity _actionstext 2e+01)
        (else
          (Widget|SetRenderOpacity _returnvalue 1.0)
          (Widget|SetRenderOpacity _actionstext 0.0)))
      (Default|CallUpdateUpgradesInfoEvent (Variables|Default|GetUpgradesInfo)))))

(event EventRemoveInfoWidget
  (bind _infowidget (Variables|Default|GetInfoWidget))
  (bind _returnvalue (UserInterface|GetUserWidgetObject _infowidget))
  (Utilities|IsValid _returnvalue
    (:Is%20Valid
      (Widget|SetRenderOpacity _returnvalue 0.0))))

(event EventRefreshInfoWidget
  (params (PlatesPlayer :type Integer))
  (bind _infoturretref (Variables|Default|GetInfoTurretRef))
  (bind _infoturretref_2 (Variables|Default|GetInfoTurretRef))
  (Utilities|IsValid (Variables|Default|GetInfoTurretRef)
    (:Is%20Valid
      (bind _returnvalue (Class|HealthComponent|GetActualHealth (Variables|Default|GetHealthComponent)))
      (if (<= _returnvalue 0.0)
        (bind _returnvalue_2 (Class|Turret|CostRepair))
        (if (>= PlatesPlayer _returnvalue_2)
          (Default|ShowActionKey _infoturretref "NewEnumerator1")
          (else
            (Default|HideActionKey _infoturretref "NewEnumerator1")))
        (Default|HideActionKey (Variables|Default|GetInfoTurretRef) "NewEnumerator0")
        (Default|HideActionKey (Variables|Default|GetInfoTurretRef) "NewEnumerator3")
        (Default|HideActionKey (Variables|Default|GetInfoTurretRef) "NewEnumerator2")
        (else
          (bind _returnvalue_3 (Class|HealthComponent|GetMaxHealth (Variables|Default|GetHealthComponent)))
          (if (>= _returnvalue _returnvalue_3)
            (Default|HideActionKey (Variables|Default|GetInfoTurretRef) "NewEnumerator1")
            (bind _returnvalue_4 (Class|Turret|GetState))
            (Default|ShowActionKey (Variables|Default|GetInfoTurretRef) "NewEnumerator0")
            (else
              (bind _returnvalue_5 (Class|Turret|CostRepair))
              (if (>= PlatesPlayer _returnvalue_5)
                (Default|ShowActionKey _infoturretref_2 "NewEnumerator1")
                (else
                  (Default|HideActionKey _infoturretref_2 "NewEnumerator1"))))))))))

(fn ConstructionScript)

(fn UpdateHealthWidget
  (bind _healthcomponent (Variables|Default|GetHealthComponent))
  (bind _healthwidgetref (Variables|Default|GetHealthWidgetRef))
  (Utilities|IsValid _healthcomponent
    (:Is%20Valid
      (bind _returnvalue (Class|HealthComponent|GetHealth _healthcomponent))
      (Utilities|IsValid _healthwidgetref
        (:Is%20Valid
          (Variables|/Game/UI/HealthLifeBars/W_TurretsHealth.W_TurretsHealth_C|SetHealth _healthwidgetref _returnvalue)
          (bind _returnvalue_2 (Class|HealthComponent|GetMaxHealth _healthcomponent))
          (Variables|/Game/UI/HealthLifeBars/W_TurretsHealth.W_TurretsHealth_C|SetMaxHealth _healthwidgetref _returnvalue_2)
          (Default|UpdateLifeText _healthwidgetref))))))